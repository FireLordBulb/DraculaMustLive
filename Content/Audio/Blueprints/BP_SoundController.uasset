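; BP_SoundController is a central audio actor that plays the game's 2D and 3D sound effects and music on request.
; Effect events map enum values to sound assets, mostly MetaSounds, through Select nodes, with many entries still unassigned.
; A MainAudio component plays and stops 2D music, while spawned music is stored in SpawnedAudio for later stopping.
; The Organ component restarts whenever it finishes, and unconnected example nodes show access via GetActorOfClass.
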(event OnAudioFinished(Organ)
  (Audio|Components|Audio|Play (Variables|Default|GetOrgan) 0.0))

(event Custom|Play%202D%20Sound%20Effect
  (params (2D%20Sound :type 2D_Sound%20Enum :default "NewEnumerator0"))
  ;[1 1 1] Play 2D sounds for the player
  (Audio|PlaySound2D (Utilities|Select :Index 2D%20Sound :NewEnumerator0 "/Game/Audio/MetaSounds/Weapon/MS_ThrowScythe.MS_ThrowScythe" :NewEnumerator1 "/Game/Audio/MetaSounds/MS_ReturnScythe.MS_ReturnScythe" :NewEnumerator2 "/Game/Audio/MetaSounds/MS_Footstep.MS_Footstep" :NewEnumerator3 "/Game/Audio/MetaSounds/MS_AmbianceBackground.MS_AmbianceBackground" :NewEnumerator4 "/Game/Audio/MetaSounds/MS_OutOfMana.MS_OutOfMana" :NewEnumerator5 "/Game/Audio/MetaSounds/MS_RaiseDead.MS_RaiseDead" :NewEnumerator6 "/Game/Audio/MetaSounds/MS_WindSpell.MS_WindSpell" :NewEnumerator7 "/Game/Audio/MetaSounds/MS_IceSpell.MS_IceSpell" :NewEnumerator8 0 :NewEnumerator9 0 :NewEnumerator10 0 :NewEnumerator11 0 :NewEnumerator12 0 :NewEnumerator13 0 :NewEnumerator17 0 :NewEnumerator14 0 :NewEnumerator15 0 :NewEnumerator16 0 :NewEnumerator18 0) 1.0 1.0 0.0 0 0 false))

(event Custom|Play%203D%20Sound%20Effect
  (params (Location :type Vector) (3D%20Sound :type 3D_Sound%20Enum :default "NewEnumerator0"))
  ;[1 1 1] Play 3D sounds for the world
  (Audio|PlaySoundatLocation (Utilities|Select :Index 3D%20Sound :NewEnumerator0 "/Game/Audio/MetaSounds/MS_Blood.MS_Blood" :NewEnumerator1 0 :NewEnumerator2 "/Game/Audio/Foley/Environment/RainAndThunder.RainAndThunder" :NewEnumerator6 "/Game/Audio/MetaSounds/MS_Footstep.MS_Footstep" :NewEnumerator7 "/Game/Audio/MetaSounds/MS_Attack.MS_Attack" :NewEnumerator8 0 :NewEnumerator9 0 :NewEnumerator10 0 :NewEnumerator11 0 :NewEnumerator12 0 :NewEnumerator13 0 :NewEnumerator14 0 :NewEnumerator15 0 :NewEnumerator16 0 :NewEnumerator17 0 :NewEnumerator18 0 :NewEnumerator19 0 :NewEnumerator20 0 :NewEnumerator21 0) Location "0, 0, 0" 1.0 1.0 0.0 0 0 0 0))

(event Custom|Stop%202D%20Music
  ;[1 1 1] 2D Music
  (Audio|Components|Audio|Stop (Variables|Default|GetMain%20Audio)))

(event Custom|Play%202D%20Music
  (params (NewSound :type Sound%20Base%20Object%20Reference))
  (bind _main_audio (Variables|Default|GetMain%20Audio))
  ;[1 1 1] 2D Music
  (Audio|Components|Audio|SetSound _main_audio NewSound)
  (Audio|Components|Audio|Play _main_audio 0.0))

(event Custom|Spawn%20Music%20at%20Location
  (params (Location :type Vector) (AttenuationSettings :type Sound%20Attenuation%20Object%20Reference) (Music :type VO_Sound%20Enum :default "NewEnumerator0"))
  ;[1 1 1] Spawned Music
  (bind _returnvalue (Audio|SpawnSoundAttached (Utilities|Select :Index Music :NewEnumerator1 "/Game/Audio/Music/Theme.Theme" :NewEnumerator0 "/Game/Audio/MetaSounds/MS_ChurchOrgan.MS_ChurchOrgan") 0 "None" Location "0, 0, 0" "KeepRelativeOffset" false 1.0 1.0 0.0 AttenuationSettings 0))
  (Variables|Default|SetSpawned%20Audio _returnvalue))

(event Custom|Stop%20Spawned%20Music
  ;[1 1 1] Spawned Music
  (Audio|Components|Audio|Stop (Variables|Default|GetSpawned%20Audio)))

(fn ConstructionScript)