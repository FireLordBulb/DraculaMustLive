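; BP_SunSet moves the level's sun, stepping its pitch each time a spawner wave ends.
; On BeginPlay it takes the first DirectionalLight found, applies a relative rotation with fixed roll and yaw, then increments the stored pitch.
; SpawnRef's OnWaveEnd event re-enters that same set-and-increment chain, so the light jumps in discrete steps rather than animating.
; An alternative SetActorRotation path is left disconnected.
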(event OnWaveEnd(SpawnRef)
  (Transformation|SetRelativeRotation (Variables|/Script/Engine.Actor|GetRootComponent (Variables|Default|Getsun)) (Math|Rotator|MakeRotator 112.0 (Variables|Default|GetNewVar) 6e+01) true false)
  (Variables|Default|SetNewVar (+ (Variables|Default|GetNewVar) 5.0)))

(event EventBeginPlay
  (bind _outactors (Actor|GetAllActorsOfClass "/Script/Engine.DirectionalLight"))
  (Variables|Default|Setsun (Utilities|Array|Get(acopy) _outactors))
  (Transformation|SetRelativeRotation (Variables|/Script/Engine.Actor|GetRootComponent (Variables|Default|Getsun)) (Math|Rotator|MakeRotator 112.0 (Variables|Default|GetNewVar) 6e+01) true false)
  (Variables|Default|SetNewVar (+ (Variables|Default|GetNewVar) 5.0)))

(fn ConstructionScript)