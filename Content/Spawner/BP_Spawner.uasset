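; BP_Spawner is a spawner that tracks which waves of the BP_SpawnerSystem it is active for.
; On BeginPlay, an empty ActiveForWaveFlags array is filled as false for indices before its Wave and true from Wave through the system's last wave.
; A non-empty flag array is left untouched, so preset per-wave patterns take priority.
; Activate is an empty function, so this Blueprint contains no spawning logic.
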(event EventBeginPlay
  (bind _wave (Variables|Default|GetWave))
  (if (Utilities|Array|IsEmpty (Variables|Default|GetActiveForWaveFlags))
    (bind _returnvalue (Actor|GetActorOfClass "/Game/Spawner/BP_SpawnerSystem.BP_SpawnerSystem_C"))
    (for _index (range 0 (- _wave 1))
      (Utilities|Array|Add (Variables|Default|GetActiveForWaveFlags) false))
    (for _index_2 (range _wave (Utilities|Array|LastIndex (Variables|/Game/Spawner/BP_SpawnerSystem.BP_SpawnerSystem_C|GetWaves _returnvalue)))
      (Utilities|Array|Add (Variables|Default|GetActiveForWaveFlags) true))))

(fn ConstructionScript)

(fn Activate)