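; Wave manager for a Dracula coffin defense game, running countdowns, enemy spawning, level unlocking and the win screen.
; Each wave splits its enemies into groups whose size varies linearly by group index, spawned in delayed batches from shuffled wave-flagged spawners under a simultaneous-enemy cap.
; Spawned enemies receive their spawner's lane.
; Clearing a wave refills player mana and starts the next countdown, destroying the next level's doors every WavesPerLevel waves.
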(event Custom|NextWaveCountdown
  (Default|ResettoFullMana (Variables|/Game/Reaper/BP_Reaper.BP_Reaper_C|GetBP_SpellResources (Variables|SpawnerSystemState|GetReaper)))
  (bind _output_get (Variables|SpawnerSystemState|SetNextWaveSecondsLeft (Variables|SpawningParameters|GetNextWaveSeconds)))
  (Default|UpdateNextWaveCountdown (Default|GetHUD (Variables|SpawnerSystemState|GetReaper)) _output_get)
  (Utilities|FlowControl|Delay 1.0 :!label _label)
  (Utilities|FlowControl|Gate false
    (:Exit
      (bind _result (Math|Integer|DecrementInt (Variables|SpawnerSystemState|GetNextWaveSecondsLeft))
        (:%20%20
          (Default|UpdateNextWaveCountdown (Default|GetHUD (Variables|SpawnerSystemState|GetReaper)) _result)
          (Math|Integer|CompareInt _result
            (:>
              (goto _label))
            (:==
              (CallFunction|NewWave)
              (Class|BPISoundManager|Play2DSFXNumber2(Message) (Game|GetGameState) 100 "NewEnumerator1"))))))))

(event Custom|PauseTimer
  (Utilities|FlowControl|Gate false) ; enters at Close
)

(event Custom|SpawnNextBatch
  (bind _currentwavespawners (Variables|SpawnerSystemState|GetCurrentWaveSpawners))
  (Utilities|Array|Shuffle _currentwavespawners)
  (bind _array_element (Utilities|Array|ForEachLoopwithBreak _currentwavespawners :!label _label)
    (:LoopBody
      (if (and (< (Utilities|Array|Length (Variables|SpawnerSystemState|GetSpawnedEnemies)) (Variables|SpawningParameters|GetMaxSimultaneousEnemies)) (> (Variables|SpawnerSystemState|GetUnspawnedEnemiesInGroup) 0))
        (Utilities|SpawnEnemy _array_element)
        (else
          (goto _label Break))))
    (:Completed
      (if (> (Variables|SpawnerSystemState|GetUnspawnedEnemies) 0)
        (if (== (Variables|SpawnerSystemState|GetUnspawnedEnemiesInGroup) 0)
          (Utilities|SetupNextGroup)
          (Utilities|FlowControl|Delay (.groupdelay (Variables|SpawnerSystemState|GetCurrentWave)))
          (else
            (Utilities|FlowControl|Delay (Variables|SpawningParameters|GetBatchSpawnDelay))))
        (CallFunction|SpawnNextBatch)))))

(event Custom|StartTimer
  (Utilities|FlowControl|Sequence
    (:then_0
      (goto _label_2 Open))
    (:then_1
      (Utilities|FlowControl|Delay 1.0 :!label _label)
      (Utilities|FlowControl|Gate false :!label _label_2
        (:Exit
          (bind _result (Math|Integer|DecrementInt (Variables|SpawnerSystemState|GetNextWaveSecondsLeft))
            (:%20%20
              (Default|UpdateNextWaveCountdown (Default|GetHUD (Variables|SpawnerSystemState|GetReaper)) _result)
              (Math|Integer|CompareInt _result
                (:>
                  (goto _label))
                (:==
                  (CallFunction|NewWave)
                  (Class|BPISoundManager|Play2DSFXNumber2(Message) (Game|GetGameState) 100 "NewEnumerator1"))))))))))

(event EventBeginPlay
  (Variables|SpawnerSystemState|SetReaper (.AsBP%20Reaper (Utilities|Casting|CastToBP_Reaper (Game|Player|GetPlayerPawn 0))))
  (bind _returnvalue (Actor|GetActorOfClass "/Game/Dracula/BP_DraculasCoffin.BP_DraculasCoffin_C"))
  (Variables|SpawnerSystemState|SetDraculasCoffin _returnvalue)
  (Utilities|FlowControl|DelayUntilNextTick)
  (bind _outactors (Actor|GetAllActorsOfClass "/Game/Spawner/BP_Spawner.BP_Spawner_C"))
  (Variables|SpawnerSystemState|SetAllSpawners _outactors)
  (CallFunction|GetSpawnersforWave)
  (CallFunction|NewWave)
  ;[0.6549 0.1303 1] Open the doors for all levels upto the starting one.
  (for _index (range 0 (/ (Variables|SpawnerSystemState|GetWaveIndex) (Variables|SpawningParameters|GetWavesPerLevel)))
    (for _array_element (.doors (Utilities|Array|Get(acopy) (Variables|SpawningParameters|GetLevels) _index))
      (Actor|DestroyActor _array_element))))

(fn ConstructionScript)

(fn NewWave
  (if (Variables|SpawnerSystemState|GetWaveIsOver)
    (Variables|SpawnerSystemState|SetWaveIsOver false)
    (CallFunction|RecalculateCurrentSplines)
    (bind _output_get (Variables|SpawnerSystemState|SetCurrentWave (Utilities|Array|Get(acopy) (Variables|SpawningParameters|GetWaves) (Variables|SpawnerSystemState|GetWaveIndex))))
    (bind _output_get_2 (Variables|SpawnerSystemState|SetUnspawnedEnemies (.enemycount _output_get)))
    (Variables|SpawnerSystemState|SetGroupIndex -1)
    (Variables|SpawnerSystemState|SetAverageGroupSize (/ _output_get_2 (Math|Conversions|ToFloat(Integer) (.groupcount _output_get))))
    (Utilities|SetupNextGroup)
    (CallFunction|SpawnNextBatch)
    (Default|UpdateWave (Default|GetHUD (Variables|SpawnerSystemState|GetReaper)) (Variables|SpawnerSystemState|GetWaveIndex))
    (Default|CallOnWaveStart)))

(fn GetSpawnersforWave
  (Utilities|Array|Clear (Variables|SpawnerSystemState|GetCurrentWaveSpawners))
  (for _array_element (Variables|SpawnerSystemState|GetAllSpawners)
    (if (Utilities|Array|Get(acopy) (Variables|/Game/Spawner/BP_Spawner.BP_Spawner_C|GetActiveForWaveFlags _array_element) (Variables|SpawnerSystemState|GetWaveIndex))
      (Utilities|Array|Add (Variables|SpawnerSystemState|GetCurrentWaveSpawners) _array_element))))

(fn OpenNewLevel
  (bind _waveindex (Variables|SpawnerSystemState|GetWaveIndex))
  (bind _wavesperlevel (Variables|SpawningParameters|GetWavesPerLevel))
  (bind _levels (Variables|SpawningParameters|GetLevels))
  (bind _returnvalue (/ _waveindex _wavesperlevel))
  (bind _output (Utilities|Array|Get(acopy) _levels _returnvalue))
  (if (== (Math|Integer|%(Integer) (Variables|SpawnerSystemState|GetWaveIndex) (Variables|SpawningParameters|GetWavesPerLevel)) 0)
    (for _array_element (.Doors (Utilities|Struct|BreakF_LevelData _output))
      (Actor|DestroyActor _array_element))
    (Default|SetText (Default|GetHUD (Variables|SpawnerSystemState|GetReaper)) "New section unlocked!")
    (Default|CallOnLevelEnd _output)))

(fn RemovefromSpawnedEnemies
  (params (Enemy :type BP%20Basic%20Enemy%20Object%20Reference))
  (bind _returnvalue (Game|GetPlayerController 0))
  (Utilities|Array|RemoveItem (Variables|SpawnerSystemState|GetSpawnedEnemies) Enemy)
  (Development|PrintString (Utilities|String|Append "Enemies left: " (Utilities|String|ToString(Integer) (+ (Utilities|Array|Length (Variables|SpawnerSystemState|GetSpawnedEnemies)) (Variables|SpawnerSystemState|GetUnspawnedEnemies)))))
  (if (== (+ (Utilities|Array|Length (Variables|SpawnerSystemState|GetSpawnedEnemies)) (Variables|SpawnerSystemState|GetUnspawnedEnemies)) 0)
    (Variables|SpawnerSystemState|SetWaveIsOver true)
    (bind _result (Math|Integer|IncrementInt (Variables|SpawnerSystemState|GetWaveIndex))
      (:%20%20
        (Math|Integer|CompareInt _result (Utilities|Array|Length (Variables|SpawningParameters|GetWaves))
          (:>
            (Development|PrintString "You won! Dracula was defended until the sun set." :!label _label)
            (bind _returnvalue_2 (UserInterface|CreateWidget "/Game/UI/WBP_WinScreen.WBP_WinScreen_C"))
            (UserInterface|Viewport|AddtoViewport _returnvalue_2 0)
            (Variables|/Script/Engine.PlayerController|SetbShowMouseCursor _returnvalue true)
            (Input|SetInputModeUIOnly _returnvalue 0 "DoNotLock" false)
            (Utilities|Time|SetGlobalTimeDilation 0.0))
          (:==
            (goto _label))
          (:<
            (CallFunction|OpenNewLevel)
            (CallFunction|GetSpawnersforWave)
            (CallFunction|NextWaveCountdown)
            (Default|CallOnWaveEnd)))))))

(fn RecalculateCurrentSplines
  (bind _currentlocationlanes (Variables|SpawnerSystemState|GetCurrentLocationLanes))
  (Utilities|Set|Clear _currentlocationlanes)
  (for _array_element (Variables|SpawnerSystemState|GetCurrentWaveSpawners)
    (Utilities|Set|Add _currentlocationlanes (Utilities|GetLane _array_element))))