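; Basic pitchfork-wielding lane enemy that attacks Dracula's coffin, minions and the player.
; Overlaps and player damage pick targets, favoring the coffin, and feed the EnemyAI blackboard; AttackTarget deals delayed montage-timed melee damage.
; Levitate polls velocity at 20 Hz to suspend it midair, then Stun and RecalculateLane snap its blackboard spline position to the nearest lane.
; A gated, retriggerable kill timer destroys stuck enemies to prevent softlocks.
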(event OnComponentBeginOverlap(EnemyAttackRange)
  (params (OverlappedComponent :type Primitive%20Component%20Object%20Reference) (OtherActor :type Actor%20Object%20Reference) (OtherComp :type Primitive%20Component%20Object%20Reference) (OtherBodyIndex :type Integer) (bFromSweep :type Boolean) (SweepResult :type Hit%20Result%20Structure%20%28by%20ref%29))
  ;[1 0.3395 0.1284] Add Target
  (if (Utilities|IsValidTarget OtherActor)
    (if (or (Utilities|IsDracula OtherActor) (<= (Math|Random|RandomFloat) (Variables|Default|GetChanceToAttack)))
      (CallFunction|SetTargettoAttack OtherActor))))

(event OnComponentEndOverlap(EnemyAttackRange)
  (params (OverlappedComponent :type Primitive%20Component%20Object%20Reference) (OtherActor :type Actor%20Object%20Reference) (OtherComp :type Primitive%20Component%20Object%20Reference) (OtherBodyIndex :type Integer))
  ;[0.237 1 0.5909] Remove Target
  (if (and (== OtherActor (Variables|Default|GetTarget)) (not (Game|IsActorBeingDestroyed)))
    (CallFunction|SetTargettoAttack)
    (CallFunction|RecalculateLane)))

(event Custom|Stun
  (params (Seconds :type Float%20%28double-precision%29))
  (CallFunction|ResetKillTimer)
  (Utilities|FlowControl|RetriggerableDelay Seconds)
  (Physics|SetSimulatePhysics (Variables|Collision|GetCapsuleComponent) false)
  (CallFunction|RecalculateLane))

(event Custom|AttackTarget
  (bind _target (Variables|Default|GetTarget))
  (bind _target_2 (Variables|Default|GetTarget))
  (bind _rootcomponent (Variables|/Script/Engine.Actor|GetRootComponent _target))
  (bind (_asprimitive_component _bsuccess) (Utilities|Casting|CastToPrimitiveComponent _rootcomponent))
  ;[1 1 1] Attacking
  (if (not (Variables|Default|GetIsAttacking))
    (Utilities|IsValid (Variables|Default|GetTarget)
      (:Is%20Valid
        (Math|Float|CompareFloat (Variables|Default|GetRadius) (Math|Float|SelectFloat (.ReturnValue (Collision|GetClosestPointonCollision _asprimitive_component (Transformation|GetActorLocation) "None")) (Transformation|GetDistanceTo (Variables|Default|GetTarget)) _bsuccess)
          (:>
            _)
          (:==
            _))
        (Variables|Default|SetIsAttacking true)
        (Class|BPISoundManager|Play3DSFX(Message) (Game|GetGameState) 100 (Transformation|GetWorldLocation (Variables|Collision|GetCapsuleComponent)) "NewEnumerator15")
        (Animation|Montage|PlayMontage (Variables|Character|GetMesh) "/Game/Enemies/Animations/AM_Attack.AM_Attack"
          (:then
            (Utilities|FlowControl|Delay 0.9)
            (Utilities|IsValid _target_2
              (:Is%20Valid
                (bind _survived (Default|TakeDamage (Actor|GetComponentbyClass _target_2 "/Game/Dracula/BP_Health.BP_Health_C") (Variables|Default|GetAttackDamage) false self))
                (Utilities|Casting|CastToBP_Reaper (Variables|Default|GetTarget)
                  (:then
                    (Class|BPISoundManager|Play2DSFXNumber2(Message) (Game|GetGameState) 100 "NewEnumerator0"))
                  (:CastFailed
                    (Class|BPISoundManager|Play3DSFX(Message) (Game|GetGameState) 100 (Transformation|GetActorLocation) "NewEnumerator10")))
                (if (not _survived)
                  (CallFunction|SetTargettoAttack)))))
          (:OnCompleted
            (Variables|Default|SetIsAttacking false)))))))

(event Custom|Levitate
  (params (LevitationSeconds :type Float%20%28double-precision%29) (StunSeconds :type Float%20%28double-precision%29))
  (bind _capsulecomponent (Variables|Collision|GetCapsuleComponent))
  (Utilities|FlowControl|Delay 0.05 :!label _label) ; Not using regular tick, 20 fps is often enough.
  (Math|Float|CompareFloat (.z (Transformation|GetVelocity)) 0.0
    (:>
      (goto _label))
    (:==
      _)
    (:<
      _))
  (Physics|SetPhysicsLinearVelocity _capsulecomponent "0, 0, 0" false "None")
  (Physics|SetEnableGravity _capsulecomponent false)
  (Utilities|FlowControl|RetriggerableDelay LevitationSeconds)
  (Physics|SetEnableGravity _capsulecomponent true)
  (CallFunction|Stun StunSeconds))

(event Custom|ResetKillTimer
  ;[1 1 1] Prevents softlock if an enemy end up out of bounds.
  (Utilities|FlowControl|Gate true
    (:Exit
      (Utilities|FlowControl|RetriggerableDelay 3e+01)
      (Actor|DestroyActor))))

(event EventBeginPlay
  ;[0.1199 0.437 0.8125] AI Setup
  (bind _output_get (Variables|Default|SetMyController (.AsEnemy%20AI (Utilities|Casting|CastToEnemyAI (AI|GetAIController self)))))
  (Default|StartAI _output_get)
  (Transformation|AttachComponentToComponent (Variables|Default|GetPitchFork) (Variables|Character|GetMesh) "indexFinger_01_l" "SnapToTarget" "KeepRelative" "KeepRelative" true)
  ;[1 1 1] Prevents softlock if an enemy end up out of bounds.
  (Utilities|FlowControl|Delay 9e+01)
  (Utilities|FlowControl|Sequence
    (:then_0
      (goto _label Open))
    (:then_1
      (Utilities|FlowControl|Gate true :!label _label
        (:Exit
          (Utilities|FlowControl|RetriggerableDelay 3e+01)
          (Actor|DestroyActor))))))

(event EventDestroyed
  (bind _spawnersystem (Variables|Default|GetSpawnerSystem))
  ;[0.3958 0 0] Destroyed
  (Utilities|IsValid _spawnersystem
    (:Is%20Valid
      (Default|RemovefromSpawnedEnemies _spawnersystem self)
      (Widget|RemovefromParent (Variables|Default|GetMapIcon)))))

(event EventSetIcon
  (params (Icon :type WBP%20Map%20Icon%20Object%20Reference))
  (Variables|Default|SetMapIcon Icon))

(event EventOnDeath
  (Actor|DestroyActor))

(event EventOnTakeDamage
  (params (HealthLeft :type Float%20%28double-precision%29) (Attacker :type Actor%20Object%20Reference))
  (Utilities|FlowControl|Sequence
    (:then_0
      (CallFunction|ResetKillTimer)
      (if (== Attacker (Game|Player|GetPlayerPawn 0))
        (Variables|Default|SetChanceToAttack (Variables|Default|GetAggroed))
        (if (<= (Math|Random|RandomFloat) (Variables|Default|GetChanceToAttack))
          (CallFunction|SetTargettoAttack (Game|Player|GetPlayerPawn 0)))))
    (:then_1
      ;[1 0.2175 0.1976] Update healthbar
      (Utilities|FlowControl|Delay 0.1)
      (Default|SetPercent (.AsWBP%20Enemy%20Health%20Bar (Utilities|Casting|CastToWBP_EnemyHealthBar (UserInterface|GetWidget (Variables|Default|GetWidget)))) (Default|GetHealthPercent (Variables|Default|GetBP_Health))))))

(fn ConstructionScript)

(fn SetTargettoAttack
  (params (TargetToAttack :type Actor%20Object%20Reference))
  (bind _mycontroller (Variables|Default|GetMyController))
  (bind _returnvalue (AI|GetBlackboard _mycontroller))
  (if (not (and (Utilities|IsValid TargetToAttack) (Utilities|IsDracula (Variables|Default|GetTarget))))
    (bind _output_get (Variables|Default|SetTarget TargetToAttack))
    (AI|Components|Blackboard|SetValueasBool _returnvalue (Utilities|Name|MakeLiteralName "TargetInRange") (Utilities|IsValid _output_get))
    (AI|Components|Blackboard|SetValueasObject _returnvalue (Utilities|Name|MakeLiteralName "TargetToAttack") _output_get)
    (AI|Components|Blackboard|SetValueasBool _returnvalue (Utilities|Name|MakeLiteralName "TargetingCoffin") (Utilities|IsDracula _output_get))
    (CallFunction|ResetKillTimer)
    (Utilities|IsValid _output_get
      (:Is%20Valid
        (bind _asprimitive_component (Utilities|Casting|CastToPrimitiveComponent (Variables|/Script/Engine.Actor|GetRootComponent _output_get))
          (:then
            (AI|Components|Blackboard|SetValueasVector _returnvalue (Utilities|Name|MakeLiteralName "TargetCollision") (.OutPointOnBody (Collision|GetClosestPointonCollision _asprimitive_component (Transformation|GetActorLocation) "None"))))
          (:CastFailed
            (AI|Components|Blackboard|SetValueasVector _returnvalue (Utilities|Name|MakeLiteralName "TargetLocation") (Transformation|GetWorldLocation (Variables|/Script/Engine.Actor|GetRootComponent _output_get)))))))))

(fn RecalculateLane
  (bind _returnvalue (Transformation|GetActorLocation))
  (bind _result (Utilities|Set|ToArray (Variables|/Game/Spawner/BP_SpawnerSystem.BP_SpawnerSystem_C|GetCurrentLocationLanes (Variables|Default|GetSpawnerSystem))))
  (for _array_element _result
    (Math|Float|CompareFloat (Math|Vector|Distance(Vector) (Spline|FindLocationClosesttoWorldLocation (Variables|/Game/Enemies/BP_Lane.BP_Lane_C|GetSpline _array_element) _returnvalue "World") _returnvalue) (LocalVariables|GetShortestDistance)
      (:<
        (LocalVariables|SetShortestDistance (Math|Vector|Distance(Vector) (Spline|FindLocationClosesttoWorldLocation (Variables|/Game/Enemies/BP_Lane.BP_Lane_C|GetSpline _array_element) _returnvalue "World") _returnvalue))
        (LocalVariables|SetClosestLane _array_element))))
  (Variables|Default|SetLane (LocalVariables|GetClosestLane))
  (AI|Components|Blackboard|SetValueasFloat (AI|GetBlackboard (Variables|Default|GetMyController)) (Utilities|Name|MakeLiteralName "SplinePosition") (/ (Class|SplineComponent|GetDistanceAlongSplineatLocation (Variables|/Game/Enemies/BP_Lane.BP_Lane_C|GetSpline (Variables|Default|GetLane)) (Spline|FindLocationClosesttoWorldLocation (Variables|/Game/Enemies/BP_Lane.BP_Lane_C|GetSpline (Variables|Default|GetLane)) (Transformation|GetActorLocation) "World") "World") (Spline|GetSplineLength (Variables|/Game/Enemies/BP_Lane.BP_Lane_C|GetSpline (Variables|Default|GetLane))))))

(fn GetIcon
  (return (Variables|Default|GetMapIcon)))