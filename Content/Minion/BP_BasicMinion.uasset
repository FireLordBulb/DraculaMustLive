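; BP_BasicMinion is a temporary allied minion, tracked in the Reaper player's spell component, that hunts BP_BasicEnemy actors and despawns after a set time.
; An aggro sphere maintains the target list; Tick picks the nearest, moves to it by AI or attacks, applying delayed damage through BP_Health.
; A game-state modifier can raise its maximum health on spawn.
; Wind-blast and levitate events toggle capsule physics and gravity, with levitation polling vertical velocity on a delay loop.
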(event OnComponentBeginOverlap(AggroRadius)
  (params (OverlappedComponent :type Primitive%20Component%20Object%20Reference) (OtherActor :type Actor%20Object%20Reference) (OtherComp :type Primitive%20Component%20Object%20Reference) (OtherBodyIndex :type Integer) (bFromSweep :type Boolean) (SweepResult :type Hit%20Result%20Structure%20%28by%20ref%29))
  (if (Utilities|ClassIsChildOf (Utilities|GetClass OtherActor) "/Game/Enemies/BP_BasicEnemy.BP_BasicEnemy_C")
    (Utilities|Array|Add (Variables|Default|GetTargetsInRange) OtherActor)
    (Class|BPISoundManager|Play3DSFX(Message) (Game|GetGameState) 100 (Transformation|GetWorldLocation (Variables|Collision|GetCapsuleComponent)) "NewEnumerator1")))

(event OnComponentEndOverlap(AggroRadius)
  (params (OverlappedComponent :type Primitive%20Component%20Object%20Reference) (OtherActor :type Actor%20Object%20Reference) (OtherComp :type Primitive%20Component%20Object%20Reference) (OtherBodyIndex :type Integer))
  (bind _targetsinrange (Variables|Default|GetTargetsInRange))
  (if (Utilities|Array|ContainsItem _targetsinrange OtherActor)
    (Utilities|Array|RemoveItem _targetsinrange (Utilities|Array|Get(acopy) _targetsinrange (Utilities|Array|FindItem _targetsinrange OtherActor)))
    (if (Utilities|Array|IsEmpty (Variables|Default|GetTargetsInRange))
      (Variables|Default|SetTargetInRange false))))

(event Custom|AttackTarget
  (bind _target (Variables|Default|GetTarget))
  (Utilities|IsValid _target
    (:Is%20Valid
      (Variables|Default|SetAttackFloat 1.0)
      (Utilities|FlowControl|Delay 1.0)
      (Variables|Default|SetAttackFloat 0.0)
      (Utilities|IsValid _target
        (:Is%20Valid
          (bind _survived (Default|TakeDamage (Actor|GetComponentbyClass _target "/Game/Dracula/BP_Health.BP_Health_C") (Variables|Default|GetDamage) false self))
          (if (not _survived)
            (Utilities|Array|RemoveItem (Variables|Default|GetTargetsInRange) _target)))))))

(event Custom|Find%20Nearest
  (if (not (Utilities|Array|IsEmpty (Variables|Default|GetTargetsInRange)))
    (Variables|Default|SetTarget (.ReturnValue (Actor|FindNearestActor (Transformation|GetActorLocation self) (Variables|Default|GetTargetsInRange))))
    (Variables|Default|SetTargetInRange true)))

(event Custom|Levitate
  (params (LevitationSeconds :type Float%20%28double-precision%29))
  (bind _capsulecomponent (Variables|Collision|GetCapsuleComponent))
  (Utilities|FlowControl|Delay 0.05 :!label _label) ; Not using regular tick, 20 fps is often enough.
  (Math|Float|CompareFloat (.z (Transformation|GetVelocity)) 0.0
    (:>
      (goto _label))
    (:==
      _)
    (:<
      _))
  (Physics|SetPhysicsLinearVelocity _capsulecomponent "0, 0, 0" false "None")
  (Physics|SetEnableGravity _capsulecomponent false)
  (Utilities|FlowControl|RetriggerableDelay LevitationSeconds)
  (Physics|SetEnableGravity _capsulecomponent true)
  (Utilities|FlowControl|Delay 2.0)
  (Physics|SetSimulatePhysics (Variables|Collision|GetCapsuleComponent) false))

(event Custom|WindBlasted
  (Utilities|FlowControl|Delay 2.0)
  (Physics|SetSimulatePhysics (Variables|Collision|GetCapsuleComponent) false))

(event EventBeginPlay
  (CallFunction|CheckforModifier)
  (Utilities|Array|Add (Variables|/Game/Reaper/BP_Spells.BP_Spells_C|GetSpawnedMinions (Variables|/Game/Reaper/BP_Reaper.BP_Reaper_C|GetBP_Spells (.AsBP%20Reaper (Utilities|Casting|CastToBP_Reaper (Game|Player|GetPlayerPawn 0))))) self)
  (CallFunction|FindNearest)
  (Utilities|DespawnMinion))

(event EventDestroyed
  (Utilities|Array|RemoveItem (Variables|/Game/Reaper/BP_Spells.BP_Spells_C|GetSpawnedMinions (Variables|/Game/Reaper/BP_Reaper.BP_Reaper_C|GetBP_Spells (.AsBP%20Reaper (Utilities|Casting|CastToBP_Reaper (Game|Player|GetPlayerPawn 0))))) self)
  (Widget|RemovefromParent (Variables|Default|GetMapIcon)))

(event EventSetIcon
  (params (Icon :type WBP%20Map%20Icon%20Object%20Reference))
  (Variables|Default|SetMapIcon Icon))

(event EventTick
  (params (DeltaSeconds :type Float%20%28single-precision%29))
  (bind _self self)
  (bind _targetsinrange (Variables|Default|GetTargetsInRange))
  (bind _returnvalue (Transformation|GetActorLocation _self))
  (bind (_distance _returnvalue_2) (Actor|FindNearestActor _returnvalue _targetsinrange))
  (CallFunction|FindNearest)
  (if (Variables|Default|GetTargetInRange)
    (if (<= _distance (Variables|Default|GetAttackRange))
      (CallFunction|AttackTarget)
      (else
        (AI|AIMoveTo self "0, 0, 0" _returnvalue_2 5e+01 false)))))

(fn ConstructionScript)

(fn SetTargettoAttack
  (params (TargetToAttack :type Actor%20Object%20Reference)))

(fn CheckforModifier
  (bind _asreaper_game_state (Utilities|Casting|CastToReaperGameState (Game|GetGameState)))
  (if (Variables|/Game/ReaperGameState.ReaperGameState_C|GetMinion_Modifier2 _asreaper_game_state)
    (Default|IncreaseMaximumHealth (Variables|Default|GetBP_Health) (Variables|Default|GetModifier_Health))))

(fn GetIcon
  (return (Variables|Default|GetMapIcon)))