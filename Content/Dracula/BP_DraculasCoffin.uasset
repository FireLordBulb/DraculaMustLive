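; Dracula's coffin actor, which relocates between unlocked teleport locations and triggers the Game Over screen when destroyed.
; The spawner's level-end event unlocks new locations, while wave-end rolls for a teleport once enough exist, raising the chance after each failed roll.
; Destinations come from a shuffled bag that excludes the current location on shuffle and refills when empty.
; Teleports broadcast start and done events around a delay; damage updates the Reaper's HUD.
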(event Custom|OnLevelEnd
  (params (NewLevel :type F%20Level%20Data%20Structure))
  (if (not (Utilities|Array|IsEmpty (.newteleportlocations NewLevel)))
    (Utilities|Array|AppendArray (Variables|Default|GetUnlockedTeleportLocations) (.newteleportlocations NewLevel))
    (Utilities|Array|AppendArray (Variables|Default|GetAvailableLocations) (.newteleportlocations NewLevel))
    (CallFunction|ShuffleLocations)))

(event Custom|OnWaveEnd
  (bind _availablelocations (Variables|Default|GetAvailableLocations))
  (bind _returnvalue (Utilities|Array|LastIndex _availablelocations))
  (Math|Integer|CompareInt (Utilities|Array|Length (Variables|Default|GetUnlockedTeleportLocations)) (Variables|Default|GetMinAvalableLocationsForTeleport)
    (:>
      (Math|Float|CompareFloat (Variables|Default|GetTeleportChance) (Math|Random|RandomFloat) :!label _label
        (:>
          (if (Utilities|Array|IsEmpty (Variables|Default|GetAvailableLocations)) :!label _label_2
            (Utilities|Array|AppendArray _availablelocations (Variables|Default|GetUnlockedTeleportLocations))
            (CallFunction|ShuffleLocations))
          (CallFunction|TeleporttoLocation (Utilities|Array|Get(acopy) _availablelocations _returnvalue))
          (Utilities|Array|RemoveIndex _availablelocations _returnvalue))
        (:==
          (goto _label_2))
        (:<
          (Variables|Default|SetTeleportChance (+ (Variables|Default|GetTeleportChance) (* (Variables|Default|GetChanceIncreasePerLocation) (Utilities|Array|Length (Variables|Default|GetUnlockedTeleportLocations)))))
          (Development|PrintString "Won't teleport, random chance failed!"))))
    (:==
      (goto _label))
    (:<
      (Development|PrintString "Won't teleport, not enough destinations unlocked"))))

(event Custom|TeleportToLocation
  (params (Location :type BP%20Teleport%20Location%20Object%20Reference))
  (bind _output_get (Variables|Default|SetCurrentLocation Location))
  (Default|CallOnTeleportStart _output_get)
  (Utilities|FlowControl|Delay 3.0)
  (Transformation|SetActorTransform (Transformation|GetActorTransform _output_get) false true)
  (Variables|Default|SetTeleportChance (Variables|Default|GetBaseTeleportChance))
  (Default|CallOnTeleportDone (Variables|Default|GetCurrentLocation)))

(event EventBeginPlay
  (Variables|Default|SetTeleportChance (Variables|Default|GetBaseTeleportChance))
  (bind _returnvalue (Game|SpawnActorfromClass "/Game/Dracula/BP_TeleportLocation.BP_TeleportLocation_C" (Transformation|GetActorTransform) "Undefined" "MultiplyWithRoot" 0 "the Mausoleum" 0))
  (bind _output_get (Variables|Default|SetCurrentLocation _returnvalue))
  (Utilities|Array|Add (Variables|Default|GetUnlockedTeleportLocations) _output_get)
  (Utilities|Array|Add (Variables|Default|GetAvailableLocations) _output_get)
  (Variables|Default|SetReaper (.AsBP%20Reaper (Utilities|Casting|CastToBP_Reaper (Game|Player|GetPlayerPawn 0))))
  (bind _returnvalue_2 (Actor|GetActorOfClass "/Game/Spawner/BP_SpawnerSystem.BP_SpawnerSystem_C"))
  (EventDispatchers|BindEventtoOnLevelEnd _returnvalue_2 (delegate Custom|OnLevelEnd))
  (EventDispatchers|AssignOnWaveEnd _returnvalue_2 (delegate Custom|OnWaveEnd)))

(event EventOnDeath
  (Actor|DestroyActor))

(event EventOnTakeDamage
  (params (HealthLeft :type Float%20%28double-precision%29) (Attacker :type Actor%20Object%20Reference))
  (Default|SetText (Default|GetHUD (Variables|Default|GetReaper)) "Dracula took damage!"))

(event EventDestroyed
  (bind _returnvalue (Game|GetPlayerController 0))
  (bind _gameoverwidget (Variables|Default|GetGameOverWidget))
  (UserInterface|Viewport|AddtoViewport _gameoverwidget 99)
  (Input|SetInputModeUIOnly _returnvalue _gameoverwidget "DoNotLock" false)
  (Variables|/Script/Engine.PlayerController|SetbShowMouseCursor _returnvalue true))

(fn ConstructionScript)

(fn AddLocations)

(fn ShuffleLocations
  (bind _availablelocations (Variables|Default|GetAvailableLocations))
  (Utilities|Array|RemoveItem _availablelocations (Variables|Default|GetCurrentLocation))
  (Utilities|Array|Shuffle _availablelocations))