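; BP_Health is a health component that tracks an actor's hit points, with healing, max increases, reset and percent queries.
; TakeDamage honours a timed invincibility window, passes damage through DefenseCalculation and reports survival and damage dealt.
; It notifies owners implementing BP_DamageTaker of hits and death, calling OnDeath on death or destroying owners without the interface.
; The diminishing-returns, capped defense formula in DefenseCalculation is left unconnected.
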(event EventBeginPlay
  (Variables|Health|SetHealthPoints (Variables|Health|GetMaxHealth))
  (bind _asbp_damage_taker (Utilities|Casting|CastToBP_DamageTaker (Components|GetOwner)))
  (Variables|Default|SetOwner _asbp_damage_taker))

(fn ReduceHealth
  (params (Amount :type Float%20%28double-precision%29))
  (bind _output_get (Variables|Health|SetHealthPoints (- (Variables|Health|GetHealthPoints) Amount)))
  (if (<= _output_get 0.0)
    (Actor|DestroyActor (Components|GetOwner))))

(fn IncreaseHealth
  (params (Amount :type Float%20%28double-precision%29))
  (if (> (+ (Variables|Health|GetHealthPoints) Amount) (Variables|Health|GetMaxHealth))
    (Variables|Health|SetHealthPoints (Variables|Health|GetMaxHealth))
    (else
      (Variables|Health|SetHealthPoints (+ (Variables|Health|GetHealthPoints) Amount)))))

(fn IncreaseMaximumHealth
  (params (Amount :type Float%20%28double-precision%29))
  (Variables|Health|SetMaxHealth (+ (Variables|Health|GetMaxHealth) Amount))
  (Variables|Health|SetHealthPoints (+ (Variables|Health|GetHealthPoints) Amount)))

(fn TakeDamage
  (params (Amount :type Float%20%28double-precision%29) (IgnoreInvincibility :type Boolean) (Attacker :type Actor%20Object%20Reference))
  (bind _owner (Variables|Default|GetOwner))
  (bind _owner_2 (Variables|Default|GetOwner))
  (bind _returnvalue (Utilities|IsValidInterface _owner_2))
  (if (<= (Variables|Health|GetHealthPoints) 0.0)
    (return false true 0.0)
    (elif (or IgnoreInvincibility (>= (Utilities|Time|GetGameTimeinSeconds) (Variables|Default|GetInvincibilityTimeEnd)))
      (bind _output_get (LocalVariables|SetPreviousHealth (Variables|Health|GetHealthPoints)))
      (bind _output_get_2 (Variables|Health|SetHealthPoints (- _output_get (Utilities|DefenseCalculation Amount))))
      (if (<= _output_get_2 0.0)
        (if _returnvalue
          (Default|OnDeath _owner)
          (Default|CallOnDeath)
          (else
            (Actor|DestroyActor (Components|GetOwner))))
        (return false false (LocalVariables|GetPreviousHealth))
        (else
          (if _returnvalue
            (Default|OnTakeDamage _owner (Variables|Health|GetHealthPoints) Attacker))
          (Variables|Default|SetInvincibilityTimeEnd (+ (Variables|Default|GetInvincibilitySeconds) (Utilities|Time|GetGameTimeinSeconds)))
          (return true false (- (LocalVariables|GetPreviousHealth) (Variables|Health|GetHealthPoints)))))
      (else
        (return true true 0.0)))))

(fn GetHealthPercent
  (return (/ (Variables|Health|GetHealthPoints) (Variables|Health|GetMaxHealth))))

(fn ResettoFullHealth
  (Variables|Health|SetHealthPoints (Variables|Health|GetMaxHealth)))