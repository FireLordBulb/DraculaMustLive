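; BP_Pausing toggles the game's pause menu from the IA_Pause input or a callable Pause event, both running the same logic.
; The toggle is ignored while the shop on the player Reaper's HUD is open.
; Pausing shows the PauseMenu widget with the cursor and Game and UI input focused on it.
; Unpausing removes the menu and restores game-only input with the cursor hidden.
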(event Custom|Pause
  (bind _returnvalue (Game|GetPlayerController 0))
  (bind _returnvalue_2 (Game|GetPlayerController 0))
  (bind _pausemenu (Variables|Default|GetPauseMenu))
  (bind _pausemenu_2 (Variables|Default|GetPauseMenu))
  (bind _returnvalue_3 (UserInterface|Viewport|IsinViewport _pausemenu))
  (if (not (Variables|/Game/UI/WBP_Shop.WBP_Shop_C|GetIsOpen (Variables|/Game/UI/WBP_PlayerHUD.WBP_PlayerHUD_C|GetShop (Default|GetHUD (Variables|Default|GetReaper)))))
    (if (Game|IsGamePaused)
      (if _returnvalue_3
        (Widget|RemovefromParent _pausemenu_2)
        (Game|SetGamePaused false)
        (Input|SetInputModeGameOnly _returnvalue_2 false)
        (Variables|/Script/Engine.PlayerController|SetbShowMouseCursor _returnvalue_2 false))
      (elif (not _returnvalue_3)
        (UserInterface|Viewport|AddtoViewport _pausemenu_2 0)
        (Game|SetGamePaused true)
        (Input|SetInputModeGameandUI _returnvalue (Variables|Default|GetPauseMenu) "DoNotLock" false false)
        (Variables|/Script/Engine.PlayerController|SetbShowMouseCursor _returnvalue true)))))

(event Input|EnhancedActionEvents|EnhancedInputActionIA_Pause
  (params (ActionValue :type Boolean) (ElapsedSeconds :type Float%20%28double-precision%29) (TriggeredSeconds :type Float%20%28double-precision%29) (InputAction :type Input%20Action%20Object%20Reference :default "/Game/Input/IA_Pause.IA_Pause"))
  (bind _returnvalue (Game|GetPlayerController 0))
  (bind _returnvalue_2 (Game|GetPlayerController 0))
  (bind _pausemenu (Variables|Default|GetPauseMenu))
  (bind _pausemenu_2 (Variables|Default|GetPauseMenu))
  (bind _returnvalue_3 (UserInterface|Viewport|IsinViewport _pausemenu))
  (:Started
    (if (not (Variables|/Game/UI/WBP_Shop.WBP_Shop_C|GetIsOpen (Variables|/Game/UI/WBP_PlayerHUD.WBP_PlayerHUD_C|GetShop (Default|GetHUD (Variables|Default|GetReaper)))))
      (if (Game|IsGamePaused)
        (if _returnvalue_3
          (Widget|RemovefromParent _pausemenu_2)
          (Game|SetGamePaused false)
          (Input|SetInputModeGameOnly _returnvalue_2 false)
          (Variables|/Script/Engine.PlayerController|SetbShowMouseCursor _returnvalue_2 false))
        (elif (not _returnvalue_3)
          (UserInterface|Viewport|AddtoViewport _pausemenu_2 0)
          (Game|SetGamePaused true)
          (Input|SetInputModeGameandUI _returnvalue (Variables|Default|GetPauseMenu) "DoNotLock" false false)
          (Variables|/Script/Engine.PlayerController|SetbShowMouseCursor _returnvalue true))))))

(event EventBeginPlay
  (Variables|Default|SetReaper (.AsBP%20Reaper (Utilities|Casting|CastToBP_Reaper (Game|Player|GetPlayerPawn 0)))))