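; BP_Currency is a Blueprint that holds a currency balance in CurrentCurrency and provides functions to add to it and spend from it.
; AddCurrency adds the given amount to the balance without any checks.
; RemoveCurrency deducts only when the remainder stays strictly above zero and returns whether it succeeded, so spending the exact balance fails.
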(fn AddCurrency
  (params (Amount :type Float%20%28double-precision%29))
  (Variables|Default|SetCurrentCurrency (+ Amount (Variables|Default|GetCurrentCurrency))))

(fn RemoveCurrency
  (params (Amount :type Float%20%28double-precision%29))
  (if (> (- (Variables|Default|GetCurrentCurrency) Amount) 0.0)
    (Variables|Default|SetCurrentCurrency (- (Variables|Default|GetCurrentCurrency) Amount))
    (return true)
    (else
      (return false))))