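; BP_Spells handles the Reaper player's spell casting, gated by unlock flags on the game state, mana and a short internal cooldown.
; Pressing input casts the selected spell at the scythe hand, either spawning its actor directly or creating a held orb.
; While input is held, aiming draws a predicted projectile path with pooled objects.
; Releasing throws the orb with the spell data.
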(event Input|EnhancedActionEvents|EnhancedInputActionIA_Spells
  (params (ActionValue :type Boolean) (ElapsedSeconds :type Float%20%28double-precision%29) (TriggeredSeconds :type Float%20%28double-precision%29) (InputAction :type Input%20Action%20Object%20Reference :default "/Game/Input/IA_Spells.IA_Spells"))
  (bind _spell (CallFunction|CurrentSpell))
  (:Started
    (if (not (Variables|SpawnOrb|GetOnInternalCooldown))
      (if (CallFunction|SpellIsUnlocked (Variables|Default|GetCurrentSpellSelected))
        (bind _cancast (Default|ConsumeManaforSpell (Variables|Default|GetSpellResourceRef) _spell))
        (if _cancast
          (CallFunction|CastSpell _spell)
          (Utilities|InternalCooldown)
          (else
            (CallFunction|SpellFail)))
        (else
          (CallFunction|SpellFail)))))
  (:Ongoing
    (Utilities|AimingTrajectory))
  (:Completed
    (CallFunction|ThrowOrb)))

(event EventBeginPlay
  (bind _asbp_reaper (Utilities|Casting|CastToBP_Reaper (Game|GetPlayerCharacter 0)))
  (Variables|Default|SetSpellResourceRef (Variables|/Game/Reaper/BP_Reaper.BP_Reaper_C|GetBP_SpellResources _asbp_reaper))
  (Variables|Default|SetBP%20Scythe%20Hand (Variables|/Game/Reaper/BP_Reaper.BP_Reaper_C|GetBP_ScytheHand _asbp_reaper))
  (bind _asreaper_game_state (Utilities|Casting|CastToReaperGameState (Game|GetGameState)))
  (Variables|Components|SetAs%20Reaper%20Game%20State _asreaper_game_state)
  (Variables|Default|SetAC%20Object%20Pool (Variables|/Game/Reaper/BP_Reaper.BP_Reaper_C|GetAC_ObjectPool _asbp_reaper))
  (Variables|Default|SetCamera (Variables|/Game/Reaper/BP_Reaper.BP_Reaper_C|GetCamera _asbp_reaper)))

(event EventTick
  (params (DeltaSeconds :type Float%20%28single-precision%29)))

(fn CurrentSpell
  (return (Utilities|Array|Get(acopy) (Variables|Default|GetSpells) (Math|Conversions|ToInteger(Byte) (Variables|Default|GetCurrentSpellSelected)))))

(fn SpellFail
  (Class|BPISoundManager|Play2DSFX(Message) (Game|GetGameState) 100 "NewEnumerator4"))

(fn CastSpell
  (params (Spell :type F%20Spell%20Data%20Structure))
  (bind (_doesuseorb _actorclass) (Utilities|Struct|BreakF_SpellData Spell))
  (bind _bp_scythe_hand (Variables|Default|GetBP%20Scythe%20Hand))
  (bind _spellspawningdistance (Variables|OrbVariables|GetSpellSpawningDistance))
  (bind _returnvalue (Transformation|GetWorldLocation _bp_scythe_hand))
  (bind _returnvalue_2 (Math|Vector|GetForwardVector _bp_scythe_hand))
  (bind _returnvalue_3 (* _returnvalue_2 _spellspawningdistance))
  (bind _returnvalue_4 (+ _returnvalue _returnvalue_3))
  (bind _returnvalue_5 (Math|Conversions|ToTransform(Vector) _returnvalue_4))
  (if _doesuseorb
    (bind _returnvalue_6 (Game|SpawnActorfromClass "/Game/Reaper/Spells/BP_SpellOrb.BP_SpellOrb_C" _returnvalue_5 "AdjustIfPossibleButAlwaysSpawn" "MultiplyWithRoot" 0 0))
    (Variables|Components|SetHeldOrb _returnvalue_6)
    (else
      (Game|SpawnActorfromClass _actorclass _returnvalue_5 "AdjustIfPossibleButAlwaysSpawn" "MultiplyWithRoot" 0 0)
      ;[0 1 0.01569 0.4] Play SFX
      (Class|BPISoundManager|Play2DSFX(Message) (Game|GetGameState) 100 (.SFX (Utilities|Struct|BreakF_SpellData Spell)))))
  (Default|CallOnSpellCast Spell)
  (if (!= (Variables|Default|GetCurrentSpellSelected) 2)
    (Variables|Default|SetAiming true)))

(fn ThrowOrb
  (Utilities|IsValid (Variables|Components|GetHeldOrb)
    (:Is%20Valid
      (Variables|Default|SetAiming false)
      (Default|Throw (Variables|Components|GetHeldOrb) (Utilities|CalculateOrbThrowForce) (CallFunction|CurrentSpell))
      (Variables|Components|SetHeldOrb 0))))

(fn SpellIsUnlocked
  (params (Spell :type Enum_PlayerSpells%20Enum :default "NewEnumerator0"))
  (bind _as_reaper_game_state (Variables|Components|GetAs%20Reaper%20Game%20State))
  (return (Utilities|Select :Index Spell :NewEnumerator0 (Variables|/Game/ReaperGameState.ReaperGameState_C|GetFrost_Main _as_reaper_game_state) :NewEnumerator1 (Variables|/Game/ReaperGameState.ReaperGameState_C|GetMinion_Main _as_reaper_game_state) :NewEnumerator2 (Variables|/Game/ReaperGameState.ReaperGameState_C|GetWind_Main _as_reaper_game_state) :NewEnumerator3 false)))