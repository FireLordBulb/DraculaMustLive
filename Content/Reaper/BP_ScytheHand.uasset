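; BP_ScytheHand is the player's scythe hand, spawning a BP_Scythe at its transform and driving it from attack input.
; Pressing starts a combo click while the scythe is held or recalled; releasing then throws it.
; Releasing while it is thrown or stuck recalls it after a delay timed from the OnThrow event.
; Holding past a threshold, less one timecode frame interval, sets a flag passed to throw and recall.
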(event Custom|SetThrowTime
  (Variables|Default|SetThrowTime (Utilities|Time|GetGameTimeinSeconds)))

(event Input|EnhancedActionEvents|EnhancedInputActionIA_ScytheAttack
  (params (ActionValue :type Boolean) (ElapsedSeconds :type Float%20%28double-precision%29) (TriggeredSeconds :type Float%20%28double-precision%29) (InputAction :type Input%20Action%20Object%20Reference :default "/Game/Input/IA_ScytheAttack.IA_ScytheAttack"))
  (bind _scythe (Variables|Default|GetScythe))
  (bind _state (Default|GetState _scythe))
  (:Started
    (switch Utilities|FlowControl|Switch|SwitchonE_ScytheState _state
      (:NewEnumerator0
        _)
      (:NewEnumerator2
        _))
    (Default|StartComboClick (Variables|Default|GetScythe)))
  (:Ongoing
    (Math|Float|CompareFloat ElapsedSeconds (- (Variables|Default|GetHoldTimeThreshold) (Class|TimeManagementBlueprintLibrary|ToInterval(FrameRate) (Class|TimeManagementBlueprintLibrary|GetTimecodeFrameRate)))
      (:>
        _)
      (:==
        _))
    (Variables|Default|SetHoldIsActive true))
  (:Completed
    (Utilities|FlowControl|Sequence
      (:then_0
        (switch Utilities|FlowControl|Switch|SwitchonE_ScytheState _state
          (:NewEnumerator0
            (Default|Throw (Variables|Default|GetScythe) (Variables|Default|GetHoldIsActive) :!label _label))
          (:NewEnumerator1
            (Math|Float|CompareFloat (Utilities|Time|GetGameTimeinSeconds) (+ (Variables|Default|GetThrowTime) (Variables|Default|GetRecallDelaySeconds)) :!label _label_2
              (:>
                (Default|Recall (Variables|Default|GetScythe) (Variables|Default|GetHoldIsActive)))))
          (:NewEnumerator4
            (goto _label_2))
          (:NewEnumerator2
            (goto _label))))
      (:then_1
        (Variables|Default|SetHoldIsActive false)))))

(event EventBeginPlay
  (bind _returnvalue (Game|SpawnActorfromClass "/Game/Reaper/BP_Scythe.BP_Scythe_C" (Transformation|GetWorldTransform) "AlwaysSpawn" "MultiplyWithRoot" 0 self (Game|Player|GetPlayerPawn 0)))
  (bind _output_get (Variables|Default|SetScythe _returnvalue))
  (EventDispatchers|BindEventtoOnThrow _output_get (delegate Custom|SetThrowTime)))

(fn ResetScythetoHeld
  (Default|MakeHeld (Variables|Default|GetScythe)))