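; Spell resource Blueprint that tracks mana and a shared cooldown for casting, with upgrades for max mana, regen rank and cooldown.
; Tick regenerates mana unless frozen, and AddMana caps it at max, notifying through CallOnManaChanged, as does spending.
; Cooldown countdown relies on an external caller.
; CalculateManaRegen contains a logarithmic rank-scaling formula, but it appears unconnected to any output.
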(event EventBeginPlay
  (Variables|ManaPoints|SetManaPoints (Variables|ManaPoints|GetMaxMana)))

(event EventTick
  (params (DeltaSeconds :type Float%20%28single-precision%29))
  (if (not (Variables|ManaRegen|GetRegenIsFrozen))
    (CallFunction|AddMana (* DeltaSeconds (Utilities|CalculateManaRegen)))))

(fn ConsumeManaforSpell
  (params (Spell :type F%20Spell%20Data%20Structure))
  (if (>= (- (Variables|ManaPoints|GetManaPoints) (.manacost Spell)) 0.0)
    (Variables|ManaPoints|SetManaPoints (- (Variables|ManaPoints|GetManaPoints) (.manacost Spell)))
    (Default|CallOnManaChanged (/ (Variables|ManaPoints|GetManaPoints) (Variables|ManaPoints|GetMaxMana)))
    (return true)
    (else
      (return false))))

(fn CastSpellCooldown
  (if (<= (Variables|Cooldown|GetCooldownTimerCounter) 0.0)
    (Variables|Cooldown|SetCooldownTimerCounter (Variables|Cooldown|GetCooldownTimer))
    (return true)
    (else
      (return false))))

(fn CooldownTimerCountdown
  (params (DeltaTime :type Float%20%28double-precision%29))
  (if (>= (Variables|Cooldown|GetCooldownTimerCounter) 0.0)
    (Variables|Cooldown|SetCooldownTimerCounter (Math|Float|Clamp(Float) (- (Variables|Cooldown|GetCooldownTimerCounter) DeltaTime) 0.0 (Variables|Cooldown|GetCooldownTimer)))))

(fn RegenMana
  (params (DeltaTime :type Float%20%28double-precision%29))
  (CallFunction|AddMana (* DeltaTime (Utilities|CalculateManaRegen))))

(fn IncreaseMaximumMana
  (params (Increased%20Mana :type Float%20%28double-precision%29))
  (bind _output_get (Variables|ManaPoints|SetMaxMana (+ (Variables|ManaPoints|GetMaxMana) Increased%20Mana)))
  (Variables|ManaPoints|SetManaPoints _output_get))

(fn IncreaseManaRegen
  (if (<= (Variables|ManaRegen|GetManaRegenCurrentRank) (Variables|ManaRegen|GetManaRegenMaxRank))
    (Variables|ManaRegen|SetManaRegenCurrentRank (+ (Variables|ManaRegen|GetManaRegenCurrentRank) 1))))

(fn ReduceMaxCooldown
  (if (<= (Variables|Cooldown|GetReduceCooldownTimerCurrentRank) (Variables|Cooldown|GetReduceCooldownTimerMaxRank))
    (Variables|Cooldown|SetReduceCooldownTimerCurrentRank (+ (Variables|Cooldown|GetReduceCooldownTimerCurrentRank) 1))
    (Variables|Cooldown|SetCooldownTimer (- (Variables|Cooldown|GetCooldownTimer) (/ (* (Variables|Cooldown|GetCooldownTimer) 2.0) (Variables|Cooldown|GetReduceCooldownTimerCurrentRank))))))

(fn ResettoFullMana
  (Variables|ManaPoints|SetManaPoints (Variables|ManaPoints|GetMaxMana)))

(fn AddMana
  (params (Amount :type Float%20%28double-precision%29))
  (Variables|ManaPoints|SetManaPoints (+ Amount (Variables|ManaPoints|GetManaPoints)))
  (if (>= (Variables|ManaPoints|GetManaPoints) (Variables|ManaPoints|GetMaxMana))
    (Skills/Talents|ResettoFullMana))
  (Default|CallOnManaChanged (/ (Variables|ManaPoints|GetManaPoints) (Variables|ManaPoints|GetMaxMana))))