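; BP_Reaper is the player character, tying together health, spell resources, scythe hand, camera and respawn components.
; BeginPlay adds the input mapping, creates the HUD and loads saved mouse sensitivity.
; Death and respawn share SetAbilityState to toggle collision, gravity, scythe and HUD visibility and swap input contexts, with respawn also refilling health and mana and resetting the scythe.
; Actor overlaps are forwarded to the scythe's dash handling.
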(event Custom|Respawn
  (CallFunction|SetAbilityState true "Visible" "/Game/Input/IM_Input.IM_Input" "/Game/Input/IM_PostDeathInput.IM_PostDeathInput")
  (Default|ResettoFullMana (Variables|Default|GetBP_SpellResources))
  (Default|ResettoFullHealth (Variables|Default|GetBP_Health))
  (Default|ResetScythetoHeld (Variables|Default|GetBP_ScytheHand)))

(event EventBeginPlay
  (Input|AddMappingContext (PlayerController|LocalPlayerSubsystems|GetEnhancedInputLocalPlayerSubsystem (Game|GetPlayerController 0)) "/Game/Input/IM_Input.IM_Input" 0 "(bIgnoreAllPressedKeysUntilRelease=True,bForceImmediately=False,bNotifyUserSettings=False)")
  (bind _returnvalue (UserInterface|CreateWidget "/Game/UI/WBP_PlayerHUD.WBP_PlayerHUD_C"))
  (bind _output_get (Variables|Default|SetHUD _returnvalue))
  (UserInterface|Viewport|AddtoViewport _output_get 0)
  (CallFunction|LoadSettings))

(event Collision|EventActorBeginOverlap
  (params (OtherActor :type Actor%20Object%20Reference))
  (Default|DashOverlap (Variables|/Game/Reaper/BP_ScytheHand.BP_ScytheHand_C|GetScythe (Variables|Default|GetBP_ScytheHand)) OtherActor))

(event EventOnDeath
  (CallFunction|SetAbilityState false "Hidden" "/Game/Input/IM_PostDeathInput.IM_PostDeathInput" "/Game/Input/IM_Input.IM_Input")
  (Default|StartRespawnTimer (Variables|Default|GetBP_ReaperRespawning)))

(fn ConstructionScript)

(fn GetHUD
  (return (Variables|Default|GetHUD)))

(fn SetAbilityState
  (params (IsEnabled :type Boolean) (Visibility :type ESlateVisibility%20Enum :default "Visible") (NewMappingContext :type Input%20Mapping%20Context%20Object%20Reference) (OldMappingContext :type Input%20Mapping%20Context%20Object%20Reference))
  (bind _returnvalue (Game|GetPlayerController 0))
  (bind _returnvalue_2 (PlayerController|LocalPlayerSubsystems|GetEnhancedInputLocalPlayerSubsystem _returnvalue))
  (Collision|SetActorEnableCollision IsEnabled)
  (Physics|SetEnableGravity (Variables|Collision|GetCapsuleComponent) IsEnabled)
  (Development|SetHiddeninGame (Variables|Default|GetBP_ScytheHand) (not IsEnabled) true)
  (Widget|SetVisibility (Variables|Default|GetHUD) Visibility)
  (Input|AddMappingContext _returnvalue_2 NewMappingContext 0 "(bIgnoreAllPressedKeysUntilRelease=True,bForceImmediately=False,bNotifyUserSettings=False)")
  (Input|RemoveMappingContext _returnvalue_2 OldMappingContext "(bIgnoreAllPressedKeysUntilRelease=True,bForceImmediately=False,bNotifyUserSettings=False)"))

(fn LoadSettings
  (bind _returnvalue (SaveGame|LoadGamefromSlot "settings"))
  (bind _asbp_setting_save_data (Utilities|Casting|CastToBP_SettingSaveData _returnvalue))
  (bind _asbp_reaper (Utilities|Casting|CastToBP_Reaper (Game|GetPlayerCharacter 0)))
  (Variables|/Game/Reaper/BP_ReaperCamera.BP_ReaperCamera_C|SetMouseSensitivity (Variables|BP_Reaper_C|GetBP_ReaperCamera _asbp_reaper) (Math|Float|Clamp(Float) (Variables|/Game/BP_SettingSaveData.BP_SettingSaveData_C|GetMouesSens _asbp_setting_save_data) 0.1)))