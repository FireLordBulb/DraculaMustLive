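; Reaper movement Blueprint that moves the player character from the IA_Moving Enhanced Input action and triggers movement sounds.
; Input is normalized, rotated by the controller's yaw for camera-relative direction, and applied as movement input scaled by WalkingAcceleration.
; Start-from-standstill and moving sounds play as 2D SFX through the GameState, sharing one availability flag that a delay resets to throttle playback.
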(event Input|EnhancedActionEvents|EnhancedInputActionIA_Moving
  (params (ActionValue :type Vector%202D%20Structure) (ElapsedSeconds :type Float%20%28double-precision%29) (TriggeredSeconds :type Float%20%28double-precision%29) (InputAction :type Input%20Action%20Object%20Reference :default "/Game/Input/IA_Moving.IA_Moving"))
  (bind _returnvalue (Game|GetPlayerController 0))
  (bind _returnvalue_2 (Class|KismetMathLibrary|NormalSafe2D ActionValue 0.1))
  (bind _returnvalue_3 (Pawn|GetControlRotation _returnvalue :!class /Script/Engine.Controller))
  (bind _returnvalue_4 (Class|KismetMathLibrary|GetRotated2D _returnvalue_2 (.yaw _returnvalue_3)))
  (Utilities|MoveStartSFX)
  (Pawn|Input|AddMovementInput (Game|GetPlayerCharacter 0) (Math|Vector|MakeVector (.x _returnvalue_4) (.y _returnvalue_4) 0.0) (Variables|Default|GetWalkingAcceleration) false)
  (Utilities|MovingSFX))