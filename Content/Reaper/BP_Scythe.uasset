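; The Reaper's throwable scythe weapon, which moves between Held, Thrown, Stuck and Recalled states.
; Tick flies it toward the crosshair target, lerps it back to the hand, or dashes the player to it.
; Overlaps damage targets, then pierce or stick based on hit rules including a dot-product graze check, and award souls for enemy kills.
; Upgrade flags add charged levitating throws, timed buffered combo throws, and dash, mana and heal bonuses.
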(event OnComponentBeginOverlap(Cylinder)
  (params (OverlappedComponent :type Primitive%20Component%20Object%20Reference) (OtherActor :type Actor%20Object%20Reference) (OtherComp :type Primitive%20Component%20Object%20Reference) (OtherBodyIndex :type Integer) (bFromSweep :type Boolean) (SweepResult :type Hit%20Result%20Structure%20%28by%20ref%29))
  (if (Utilities|Enum|Equal(Enum) (Variables|ScytheState|GetState) "NewEnumerator1")
    ;[1 0.629 0.1099] Getting stuck in a static object.
    (CallFunction|MakeStuck)
    (Default|CallOnStuck OtherActor)))

(event OnComponentBeginOverlap(Mesh)
  (params (OverlappedComponent :type Primitive%20Component%20Object%20Reference) (OtherActor :type Actor%20Object%20Reference) (OtherComp :type Primitive%20Component%20Object%20Reference) (OtherBodyIndex :type Integer) (bFromSweep :type Boolean) (SweepResult :type Hit%20Result%20Structure%20%28by%20ref%29))
  (bind (_shouldpierce _damage _healthcomponent _canhit) (Utilities|CheckifCanHit (Variables|ScytheState|GetOtherActor)))
  (Utilities|SaveCollisionValues OtherActor false)
  (if _canhit
    (if (Utilities|Array|ContainsItem (Variables|ScytheState|GetLargerMeshHitEnemies) (Variables|ScytheState|GetOtherActor))
      (if (Variables|UpgradeState|GetCha_CollisionIsLargerMesh) :!label _label
        (Utilities|Array|Add (Variables|ScytheState|GetLargerMeshHitEnemies) (Variables|ScytheState|GetOtherActor))
        (elif _shouldpierce
          (Utilities|Array|Add (Variables|ScytheState|GetPiercedEnemies) (Variables|ScytheState|GetOtherActor))
          (else
            ;[0.1898 1 0.3923] Getting stuck in an enemy.
            (Transformation|AttachActorToActor (Variables|ScytheState|GetOtherActor) "None" "KeepWorld" "KeepWorld" "KeepWorld" false)
            (CallFunction|MakeStuck))))
      (else
        (Default|CallOnDamage (Transformation|GetActorLocation) (Variables|ScytheState|GetOtherActor))
        (Utilities|HurtActor (Variables|ScytheState|GetOtherActor) _damage _healthcomponent
          (:Survived
            (goto _label))
          (:Died
            (Utilities|IfIsEnemy (Variables|ScytheState|GetOtherActor)
              (:then
                (Default|AddCurrency (Variables|/Game/Reaper/BP_Reaper.BP_Reaper_C|GetBP_Currency (Variables|ScytheState|GetReaper)) (Variables|SoulParameters|GetSoulsPerKill))))))))))

(event OnComponentBeginOverlap(LargerMesh)
  (params (OverlappedComponent :type Primitive%20Component%20Object%20Reference) (OtherActor :type Actor%20Object%20Reference) (OtherComp :type Primitive%20Component%20Object%20Reference) (OtherBodyIndex :type Integer) (bFromSweep :type Boolean) (SweepResult :type Hit%20Result%20Structure%20%28by%20ref%29))
  (bind (_shouldpierce _damage _healthcomponent _canhit) (Utilities|CheckifCanHit (Variables|ScytheState|GetOtherActor)))
  (Utilities|SaveCollisionValues OtherActor true)
  (if _canhit
    (if (Utilities|Array|ContainsItem (Variables|ScytheState|GetLargerMeshHitEnemies) (Variables|ScytheState|GetOtherActor))
      (if (Variables|UpgradeState|GetCha_CollisionIsLargerMesh) :!label _label
        (Utilities|Array|Add (Variables|ScytheState|GetLargerMeshHitEnemies) (Variables|ScytheState|GetOtherActor))
        (elif _shouldpierce
          (Utilities|Array|Add (Variables|ScytheState|GetPiercedEnemies) (Variables|ScytheState|GetOtherActor))
          (else
            ;[0.1898 1 0.3923] Getting stuck in an enemy.
            (Transformation|AttachActorToActor (Variables|ScytheState|GetOtherActor) "None" "KeepWorld" "KeepWorld" "KeepWorld" false)
            (CallFunction|MakeStuck))))
      (else
        (Default|CallOnDamage (Transformation|GetActorLocation) (Variables|ScytheState|GetOtherActor))
        (Utilities|HurtActor (Variables|ScytheState|GetOtherActor) _damage _healthcomponent
          (:Survived
            (goto _label))
          (:Died
            (Utilities|IfIsEnemy (Variables|ScytheState|GetOtherActor)
              (:then
                (Default|AddCurrency (Variables|/Game/Reaper/BP_Reaper.BP_Reaper_C|GetBP_Currency (Variables|ScytheState|GetReaper)) (Variables|SoulParameters|GetSoulsPerKill))))))))))

(event Custom|MovementSpeedIncrease
  (bind _reaper (Variables|ScytheState|GetReaper))
  (bind _charactermovement (Variables|/Script/Engine.Character|GetCharacterMovement _reaper))
  (Variables|/Script/Engine.CharacterMovementComponent|SetMaxWalkSpeed _charactermovement (* (Variables|UpgradeState|GetDash_DefaultWalkSpeed) (Variables|UpgradeParameters|GetDash_MoveSpeedScalar)))
  (Utilities|FlowControl|Delay (Variables|UpgradeParameters|GetDash_MoveSpeedSeconds))
  (Variables|/Script/Engine.CharacterMovementComponent|SetMaxWalkSpeed _charactermovement (Variables|UpgradeState|GetDash_DefaultWalkSpeed)))

(event EventBeginPlay
  (Variables|UpgradeState|SetDash_NormalCollisionProfile (Collision|GetCollisionProfileName (Variables|/Script/Engine.Character|GetCapsuleComponent (Game|GetPlayerCharacter 0))))
  (CallFunction|MakeHeld)
  (Variables|ScytheState|SetReaper (.AsBP%20Reaper (Utilities|Casting|CastToBP_Reaper (Game|Player|GetPlayerPawn 0))))
  (Variables|UpgradeState|SetDash_DefaultWalkSpeed (Variables|/Script/Engine.CharacterMovementComponent|GetMaxWalkSpeed (Variables|/Script/Engine.Character|GetCharacterMovement (Variables|ScytheState|GetReaper)))))

(event EventTick
  (params (DeltaSeconds :type Float%20%28single-precision%29))
  (bind (_alpha _newlocation) (Utilities|ComputeRecallNewLocation DeltaSeconds))
  (Utilities|FlowControl|Sequence
    (:then_0
      (if (Variables|UpgradeState|GetDash_IsActive)
        (Utilities|MakePlayerDash DeltaSeconds
          (:DashEnded
            (if (Variables|ScytheUpgrades|GetHasUpgradeDash_Speed)
              (CallFunction|MovementSpeedIncrease))
            ;[0.09046 0.6954 1] Catching the Scythe to hold it again.
            (CallFunction|MakeHeld :!label _label)
            (Variables|UpgradeState|SetSeq_LatestInputTime (+ (Utilities|Time|GetGameTimeinSeconds) (Variables|UpgradeParameters|GetSeq_PostCatchTimeWindow)))
            (CallFunction|DisableDash)
            (Default|CallOnCatch)
            ;[1 0.2887 0.07785] Buffered Sequential Attack
            (if (Variables|UpgradeState|GetSeq_IsActive)
              (CallFunction|Throw false))))))
    (:then_1
      (switch Utilities|FlowControl|Switch|SwitchonE_ScytheState (Variables|ScytheState|GetState)
        (:NewEnumerator0)
        (:NewEnumerator1
          (Transformation|AddActorWorldOffset (* (Variables|ScytheState|GetMoveDirection) (Variables|ScytheBaseParameters|GetFlySpeed) (Utilities|SpeedScalar) DeltaSeconds) true))
        (:NewEnumerator4)
        (:NewEnumerator2
          (Math|Float|CompareFloat _alpha (Variables|ScytheBaseParameters|GetRecallCloseEnoughAlpha)
            (:>
              (Transformation|SetActorLocation _newlocation true false))
            (:==
              (goto _label))
            (:<
              (goto _label)))))
      (Utilities|SpinScythe DeltaSeconds))))

(fn ConstructionScript)

(fn Throw
  (params (HoldIsActive :type Boolean))
  (bind _hasupgradechargedattack (Variables|ScytheUpgrades|GetHasUpgradeChargedAttack))
  (bind _returnvalue (and HoldIsActive _hasupgradechargedattack))
  (if (and (or _returnvalue (Utilities|IsinComboWindow)) (Variables|UpgradeState|GetSeq_ComboClickWasStarted))
    (Variables|UpgradeState|SetSeq_IsActive true))
  (if (Utilities|Enum|Equal(Enum) (Variables|ScytheState|GetState) "NewEnumerator0")
    (if _returnvalue
      (CallFunction|ChargedThrow))
    (Utilities|StartMoving "NewEnumerator1" 1)
    (bind _rotation (Utilities|GetCrosshairTargetRotation))
    (Transformation|SetActorRotation (Math|Rotator|MakeRotator (Variables|ScytheBaseParameters|GetThrowRollAngle) (.Pitch (Math|Rotator|BreakRotator _rotation)) (.Yaw (Math|Rotator|BreakRotator _rotation))))
    (Variables|ScytheState|SetMoveDirection (Transformation|GetActorForwardVector))
    (Collision|SetActorEnableCollision true)
    (Variables|UpgradeState|SetSeq_ComboClickWasStarted false)
    (Variables|UpgradeState|SetSeq_ClickedTooEarly false)
    (Default|CallOnThrow)
    (if (Variables|UpgradeState|GetSeq_IsActive)
      (Default|CallOnComboThrow))))

(fn Recall
  (params (HoldIsActive :type Boolean))
  (bind _returnvalue (Game|GetPlayerCharacter 0))
  (if (and HoldIsActive (Variables|ScytheUpgrades|GetHasUpgradeDash))
    (Variables|UpgradeState|SetDash_IsActive true)
    (Pawn|Components|CharacterMovement|DisableMovement (Variables|/Script/Engine.Character|GetCharacterMovement _returnvalue))
    (Collision|SetCollisionProfileName (Variables|/Script/Engine.Character|GetCapsuleComponent _returnvalue) (Variables|UpgradeParameters|GetDash_DashingCollisionProfile) false :!class /Script/Engine.PrimitiveComponent)
    (Default|CallOnBeginDash)
    (else
      (Utilities|StartMoving "NewEnumerator2" -1)
      (Variables|UpgradeState|SetSeq_IsActive false)
      (CallFunction|EndChargedThrow))))

(fn StartComboClick
  (if (Math|Boolean|ANDBoolean (Variables|ScytheUpgrades|GetHasUpgradeSequentialAttack) (not (Variables|UpgradeState|GetSeq_ClickedTooEarly)) (Utilities|IsinComboWindow))
    (Variables|UpgradeState|SetSeq_ComboClickWasStarted true)
    (else
      (Variables|UpgradeState|SetSeq_ClickedTooEarly true))))

(fn MakeHeld
  (Variables|ScytheState|SetState "NewEnumerator0")
  (Transformation|AttachComponentToComponent (Variables|Default|GetScytheHand) "None" "SnapToTarget" "SnapToTarget" "KeepWorld" false)
  (Collision|SetActorEnableCollision false))

(fn MakeStuck
  (Variables|ScytheState|SetState "NewEnumerator4")
  (CallFunction|EndChargedThrow))

(fn ChargedThrow
  (bind _largermesh (Variables|Default|GetLargerMesh))
  (Variables|UpgradeState|SetCha_IsActive true)
  (if (Variables|ScytheUpgrades|GetHasUpgradeCha_Range)
    (Collision|SetCollisionEnabled _largermesh "QueryOnly")
    (Rendering|SetVisibility _largermesh true false)))

(fn EndChargedThrow
  (bind _largermesh (Variables|Default|GetLargerMesh))
  (Variables|UpgradeState|SetCha_IsActive false)
  (if (Variables|ScytheUpgrades|GetHasUpgradeCha_Range)
    (Collision|SetCollisionEnabled _largermesh "NoCollision")
    (Rendering|SetVisibility _largermesh false false)))

(fn DisableDash
  (bind _returnvalue (Game|GetPlayerCharacter 0))
  (if (Variables|UpgradeState|GetDash_IsActive)
    (Variables|UpgradeState|SetDash_IsActive false)
    (Collision|SetCollisionProfileName (Variables|/Script/Engine.Character|GetCapsuleComponent _returnvalue) (Variables|UpgradeState|GetDash_NormalCollisionProfile) true :!class /Script/Engine.PrimitiveComponent)
    (Pawn|Components|CharacterMovement|SetMovementMode (Variables|/Script/Engine.Character|GetCharacterMovement _returnvalue) "MOVE_Walking" 0)
    (CallFunction|UnstuckfromGround)
    (Default|CallOnEndDash)))

(fn DashOverlap
  (params (OtherActor :type Actor%20Object%20Reference))
  (bind _returnvalue (Actor|GetComponentbyClass OtherActor "/Game/Dracula/BP_Health.BP_Health_C"))
  (if (Variables|UpgradeState|GetDash_IsActive)
    (if (and (Utilities|IsValid _returnvalue) (Utilities|ClassIsChildOf (Utilities|GetClass OtherActor) "/Script/Engine.Pawn"))
      (Default|CallOnDashDamage (Transformation|GetActorLocation (Variables|ScytheState|GetReaper)))
      (Utilities|HurtActor OtherActor (Variables|UpgradeParameters|GetDash_Damage) _returnvalue))))

(fn UnstuckfromGround
  (bind _returnvalue (Game|GetPlayerCharacter 0))
  (bind _returnvalue_2 (Game|GetPlayerCharacter 0))
  (bind _returnvalue_3 (Transformation|GetActorLocation _returnvalue_2))
  (bind _capsulecomponent (Variables|/Script/Engine.Character|GetCapsuleComponent _returnvalue))
  (bind _returnvalue_4 (Transformation|GetWorldLocation _capsulecomponent))
  (bind _capsulehalfheight (Variables|/Script/Engine.CapsuleComponent|GetCapsuleHalfHeight _capsulecomponent))
  (bind _returnvalue_5 (Math|Vector|MakeVector 0.0 0.0 _capsulehalfheight))
  (bind _outhit (Class|KismetSystemLibrary|LineTraceSinglebyProfile (+ _returnvalue_4 (/ _returnvalue_5 2.0)) (- _returnvalue_4 _returnvalue_5) "BlockOnlyGround" false (Utilities|Array|MakeArray _returnvalue) "None" true))
  (if (.bblockinghit _outhit)
    (Transformation|SetActorLocation _returnvalue_2 (Math|Vector|MakeVector (.x _returnvalue_3) (.y _returnvalue_3) (+ (.z (.location _outhit)) (Variables|/Script/Engine.CapsuleComponent|GetCapsuleHalfHeight (Variables|/Script/Engine.Character|GetCapsuleComponent _returnvalue_2)))) false false)))

(fn LiftActorifChargedAttack
  (params (Actor :type Actor%20Object%20Reference))
  (bind _hasupgradecha_time (Variables|ScytheUpgrades|GetHasUpgradeCha_Time))
  (bind _cha_levitationseconds (Variables|UpgradeParameters|GetCha_LevitationSeconds))
  (bind _cha_increasedlevitationseconds (Variables|UpgradeParameters|GetCha_IncreasedLevitationSeconds))
  (bind _returnvalue (Math|Float|SelectFloat _cha_increasedlevitationseconds _cha_levitationseconds _hasupgradecha_time))
  (if (Variables|UpgradeState|GetCha_IsActive)
    (bind _ascharacter (Utilities|Casting|CastToCharacter Actor))
    (Physics|SetPhysicsLinearVelocity (Variables|/Script/Engine.Character|GetCapsuleComponent _ascharacter) "0, 0, 0" false "None")
    (Physics|SetSimulatePhysics (Variables|/Script/Engine.Character|GetCapsuleComponent _ascharacter) true)
    (Physics|AddImpulse (Variables|/Script/Engine.Character|GetCapsuleComponent _ascharacter) (Math|Vector|MakeVector 0.0 0.0 (Variables|UpgradeParameters|GetCha_Impulse)) "None" false)
    (bind _asbp_basic_enemy (Utilities|Casting|CastToBP_BasicEnemy _ascharacter)
      (:then
        (Default|Levitate _asbp_basic_enemy _returnvalue (Variables|UpgradeParameters|GetCha_StunSeconds)))
      (:CastFailed
        (bind _asbp_basic_minion (Utilities|Casting|CastToBP_BasicMinion _ascharacter))
        (Default|Levitate _asbp_basic_minion _returnvalue)))))

(fn GetState
  (return (Variables|ScytheState|GetState)))

(fn DamageNumber
  (params (Location :type Vector) (Damage :type Float%20%28double-precision%29) (Color :type Linear%20Color%20Structure))
  (bind (_x _y _z) (Math|Vector|BreakVector Location))
  (bind _returnvalue (Game|SpawnActorfromClass "/Game/UI/SubWidgets/BP_DamageNumber.BP_DamageNumber_C" (Math|Transform|MakeTransform (Math|Vector|MakeVector _x _y (+ _z 1.4e+02)) "0, 0, 0" "1.000000,1.000000,1.000000") "Undefined" "MultiplyWithRoot" 0 0))
  (Default|SetText (.AsWBP%20Damage%20Number (Utilities|Casting|CastToWBP_DamageNumber (UserInterface|GetWidget (Variables|/Game/UI/SubWidgets/BP_DamageNumber.BP_DamageNumber_C|GetWidget _returnvalue)))) (Utilities|Text|ToText(Integer) (Math|Float|Ceil Damage)))
  (Appearance|SetColorandOpacity (.AsWBP%20Damage%20Number (Utilities|Casting|CastToWBP_DamageNumber (UserInterface|GetWidget (Variables|/Game/UI/SubWidgets/BP_DamageNumber.BP_DamageNumber_C|GetWidget _returnvalue)))) Color :!class /Script/UMG.UserWidget))