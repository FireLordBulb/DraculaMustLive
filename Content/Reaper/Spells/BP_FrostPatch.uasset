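; Frost patch spell actor that grows on spawn, then destroys itself when its lifetime runs out.
; BeginPlay applies game-state frost modifiers, tilts the patch using four downward traces, and scales the mesh via a timeline.
; Overlapping enemies get walk speed from CalculatePercent, whose calculation is unwired, and play a sound.
; Exiting enemies get back the speed saved in one shared variable, overwritten by each new overlap.
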(event OnComponentBeginOverlap(Sphere)
  (params (OverlappedComponent :type Primitive%20Component%20Object%20Reference) (OtherActor :type Actor%20Object%20Reference) (OtherComp :type Primitive%20Component%20Object%20Reference) (OtherBodyIndex :type Integer) (bFromSweep :type Boolean) (SweepResult :type Hit%20Result%20Structure%20%28by%20ref%29))
  (bind _asbp_basic_enemy (Utilities|Casting|CastToBP_BasicEnemy OtherActor))
  (Variables|Default|SetOriginalMaxSpeed (Variables|/Script/Engine.CharacterMovementComponent|GetMaxWalkSpeed (Variables|/Script/Engine.Character|GetCharacterMovement _asbp_basic_enemy)))
  (Variables|/Script/Engine.CharacterMovementComponent|SetMaxWalkSpeed (Variables|/Script/Engine.Character|GetCharacterMovement _asbp_basic_enemy) (Utilities|CalculatePercent (Variables|/Script/Engine.CharacterMovementComponent|GetMaxWalkSpeed (Variables|/Script/Engine.Character|GetCharacterMovement _asbp_basic_enemy))))
  (Class|BPISoundManager|Play3DSFX(Message) (Game|GetGameState) 100 (Transformation|GetWorldLocation (Variables|Default|GetDefaultSceneRoot)) "NewEnumerator11"))

(event EventBeginPlay
  (CallFunction|CheckforModifiers)
  (CallFunction|Rotation)
  (bind _growth (Timeline|Growing Play)
    (:Update
      (Transformation|SetRelativeScale3D (Variables|Default|GetStaticMesh) (Math|Vector|MakeVector (* (Variables|Default|GetGrowthModifier) _growth) (* (Variables|Default|GetGrowthModifier) _growth) (.z (Class|Actor|GetActorRelativeScale3D)))))
    (:Finished
      (Utilities|FlowControl|Gate true) ; enters at Open
    )))

(event EventTick
  (params (DeltaSeconds :type Float%20%28single-precision%29))
  (Utilities|FlowControl|Gate true
    (:Exit
      (Variables|Default|SetLifetime (- (Variables|Default|GetLifetime) DeltaSeconds))
      (if (<= (Variables|Default|GetLifetime) 0.0)
        (Actor|DestroyActor)))))

(event Collision|EventActorEndOverlap
  (params (OtherActor :type Actor%20Object%20Reference))
  (bind _asbp_basic_enemy (Utilities|Casting|CastToBP_BasicEnemy OtherActor))
  (Variables|/Script/Engine.CharacterMovementComponent|SetMaxWalkSpeed (Variables|/Script/Engine.Character|GetCharacterMovement _asbp_basic_enemy) (Variables|Default|GetOriginalMaxSpeed)))

(fn ConstructionScript
  (bind _spawnsize (Variables|Default|GetSpawnSize))
  (Transformation|SetRelativeScale3D (Variables|Default|GetStaticMesh) (Math|Vector|MakeVector _spawnsize _spawnsize (.z (Class|Actor|GetActorRelativeScale3D)))))

(fn Rotation
  (bind _linetracevalues (Variables|Default|GetLineTraceValues))
  (Variables|Default|SetLineTracePoints (Utilities|Array|MakeArray (Variables|Default|GetSphere1) (Variables|Default|GetSphere2) (Variables|Default|GetSphere3) (Variables|Default|GetSphere4)))
  (for _array_element (Variables|Default|GetLineTracePoints)
    (bind _outhit (Collision|LineTraceByChannel (Transformation|GetWorldLocation _array_element) (+ (Transformation|GetWorldLocation _array_element) (* (Math|Vector|GetUpVector (Transformation|GetWorldRotation _array_element)) -5e+02)) "TraceTypeQuery1" false 0 "ForDuration"))
    (Utilities|Array|Add (Variables|Default|GetLineTraceValues) (.Distance (Collision|BreakHitResult _outhit))))
  (Transformation|SetActorRotation (Math|Rotator|MakeRotator (- (Utilities|Array|Get(acopy) _linetracevalues) (Utilities|Array|Get(acopy) _linetracevalues 1)) (- (Utilities|Array|Get(acopy) _linetracevalues 3) (Utilities|Array|Get(acopy) _linetracevalues 2)) 0.0)))

(fn CheckforModifiers
  (bind _asreaper_game_state (Utilities|Casting|CastToReaperGameState (Game|GetGameState)))
  (if (Variables|/Game/ReaperGameState.ReaperGameState_C|GetFrost_Modifier1 _asreaper_game_state)
    (Variables|Default|SetGrowthModifier (Variables|Default|GetModifier_IncreaseRange)))
  (if (Variables|/Game/ReaperGameState.ReaperGameState_C|GetFrost_Modifier2 _asreaper_game_state)
    (Variables|Default|SetSlowdownAmount (Variables|Default|GetModifier_IncreaseSlowdown))))