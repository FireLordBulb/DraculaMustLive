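; Actor pool component in the Reaper spells folder that reuses actors instead of spawning new ones on demand.
; On BeginPlay it pre-spawns actors of the pooled class up to the pool size and marks each as not in use.
; SpawnFromPool finds the first free actor, moves it to the requested transform and marks it in use, or prints a warning when none is available.
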(event Custom|InitializePool
  (for _index (range 0 (Variables|Default|GetPoolSize))
    (bind _returnvalue (Game|SpawnActorfromClass (Variables|Default|GetPooledActorClass) (Math|Transform|MakeTransform "0, 0, 0" "0, 0, 0" "1.000000,1.000000,1.000000") "Undefined" "MultiplyWithRoot" 0 1.0 0))
    (Utilities|Array|AddUnique (Variables|Default|GetObjectPool) _returnvalue)
    (Default|SetinUse _returnvalue false)))

(event EventBeginPlay
  (CallFunction|InitializePool))

(fn FindFirstAvailableActor
  (for _array_element (Variables|Default|GetObjectPool)
    (if (not (Variables|/Game/Reaper/Spells/BP_PooledActor.BP_PooledActor_C|GetInUse _array_element))
      (return _array_element))))

(fn SpawnfromPool
  (params (SpawnTransform :type Transform))
  (bind _pooled_actor (CallFunction|FindFirstAvailableActor))
  (Utilities|IsValid _pooled_actor
    (:Is%20Valid
      (Transformation|SetActorTransform _pooled_actor SpawnTransform)
      (Default|SetinUse _pooled_actor true)
      (return _pooled_actor))
    (:Is%20Not%20Valid
      (Development|PrintString "Pool is empty"))))