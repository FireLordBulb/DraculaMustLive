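; BP_SpellOrb is a throwable spell projectile that attaches to the player Reaper's scythe hand on BeginPlay.
; Throw stores the spell data, enables physics on the sphere, launches it at the given velocity and destroys it after a lifetime delay.
; Hitting a component of the first custom collision object type spawns the spell's actor at the impact point, plays its SFX via the GameState and destroys the orb.
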(event Custom|Throw
  (params (Force :type Vector) (Spell :type F%20Spell%20Data%20Structure))
  (bind _sphere (Variables|Default|GetSphere))
  (Variables|Default|SetSpell Spell)
  (Physics|SetSimulatePhysics _sphere true)
  (Physics|SetPhysicsLinearVelocity _sphere Force false "None")
  (Utilities|FlowControl|Delay (Variables|Default|GetLifetime))
  (Actor|DestroyActor))

(event EventBeginPlay
  (bind _asbp_reaper (Utilities|Casting|CastToBP_Reaper (Game|GetPlayerCharacter 0)))
  (Transformation|AttachComponentToComponent (Variables|Default|GetSphere) (Variables|/Game/Reaper/BP_Reaper.BP_Reaper_C|GetBP_ScytheHand _asbp_reaper) "None" "KeepRelative" "SnapToTarget" "KeepRelative" true))

(event Collision|EventHit
  (params (MyComp :type Primitive%20Component%20Object%20Reference) (Other :type Actor%20Object%20Reference) (OtherComp :type Primitive%20Component%20Object%20Reference) (bSelfMoved :type Boolean) (HitLocation :type Vector :default "0, 0, 0") (HitNormal :type Vector :default "0, 0, 0") (NormalImpulse :type Vector :default "0, 0, 0") (Hit :type Hit%20Result%20Structure%20%28by%20ref%29))
  (if (Utilities|Enum|Equal(Enum) (Collision|GetCollisionObjectType OtherComp) "ECC_GameTraceChannel1")
    (Game|SpawnActorfromClass (.actorclass (Variables|Default|GetSpell)) (Math|Conversions|ToTransform(Vector) HitLocation) "Undefined" "MultiplyWithRoot" 0 0)
    ;[0 1 0.01569 0.4] Play SFX
    (Class|BPISoundManager|Play2DSFX(Message) (Game|GetGameState) 100 (.sfx (Variables|Default|GetSpell)))
    (Actor|DestroyActor)))

(fn ConstructionScript)