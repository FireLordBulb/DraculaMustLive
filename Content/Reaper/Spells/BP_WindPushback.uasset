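; Reaper wind spell actor that spawns ahead of the player's camera and knocks back enemies and minions it overlaps.
; Each tick it moves along the live camera forward vector, decays its knockback strength and expires after a set duration.
; Overlaps stun basic enemies or wind-blast minions, then enable capsule physics and apply an impulse.
; ReaperGameState modifiers override duration and knockback; the Pushback trace helper is never called here.
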(event EventBeginPlay
  (CallFunction|CheckforModifiers)
  (bind _asbp_reaper (Utilities|Casting|CastToBP_Reaper (Game|GetPlayerCharacter 0)))
  (Transformation|SetActorLocationAndRotation (+ (Transformation|GetActorLocation _asbp_reaper) (* (Math|Vector|GetForwardVector (Variables|/Game/Reaper/BP_Reaper.BP_Reaper_C|GetCamera _asbp_reaper)) (Variables|Spawn|GetStartingDistance))) (Math|Conversions|RotationFromXVector (Math|Vector|GetForwardVector (Variables|/Game/Reaper/BP_Reaper.BP_Reaper_C|GetCamera _asbp_reaper))))
  (Variables|Default|SetSpawned true))

(event Collision|EventActorBeginOverlap
  (params (OtherActor :type Actor%20Object%20Reference))
  (bind _asbp_basic_enemy (Utilities|Casting|CastToBP_BasicEnemy OtherActor)
    (:then
      (Default|Stun _asbp_basic_enemy (Variables|SpellValues|GetStunSeconds))
      (Physics|SetSimulatePhysics (Variables|/Script/Engine.Character|GetCapsuleComponent _asbp_basic_enemy) true)
      (Physics|AddImpulse (Variables|/Script/Engine.Character|GetCapsuleComponent _asbp_basic_enemy) (* (Transformation|GetActorForwardVector) (Variables|SpellValues|GetKnockbackStrength)) "None" false))
    (:CastFailed
      (bind _asbp_basic_minion (Utilities|Casting|CastToBP_BasicMinion OtherActor))
      (Default|WindBlasted _asbp_basic_minion)
      (Physics|SetSimulatePhysics (Variables|/Script/Engine.Character|GetCapsuleComponent _asbp_basic_minion) true)
      (Physics|AddImpulse (Variables|/Script/Engine.Character|GetCapsuleComponent _asbp_basic_minion) (* (Transformation|GetActorForwardVector) (Variables|SpellValues|GetKnockbackStrength)) "None" false))))

(event EventTick
  (params (DeltaSeconds :type Float%20%28single-precision%29))
  (CallFunction|DurationTimer DeltaSeconds)
  (if (Variables|Default|GetSpawned)
    (Transformation|AddActorWorldOffset (* (Math|Vector|GetForwardVector (Variables|/Game/Reaper/BP_Reaper.BP_Reaper_C|GetCamera (stale EventBeginPlay _asbp_reaper))) (Variables|SpellValues|GetSpellDistance)))))

(fn ConstructionScript)

(fn DurationTimer
  (params (DeltaTime :type Float%20%28double-precision%29))
  (Variables|SpellValues|SetSpellDuration (- (Variables|SpellValues|GetSpellDuration) DeltaTime))
  (CallFunction|ReduceKnockbackonRange DeltaTime)
  (if (<= (Variables|SpellValues|GetSpellDuration) 0.0)
    (Actor|DestroyActor)))

(fn ReduceKnockbackonRange
  (params (DeltaTime :type Float%20%28double-precision%29))
  (Variables|SpellValues|SetKnockbackStrength (- (Variables|SpellValues|GetKnockbackStrength) (* (* DeltaTime 5.0) (Variables|SpellValues|GetKnockbackStrength)))))

(fn Pushback
  (params (Target :type Actor%20Object%20Reference))
  (bind _returnvalue (Game|GetPlayerCharacter 0))
  (bind _returnvalue_2 (Collision|LineTraceByChannel (Transformation|GetActorLocation Target) (Transformation|GetActorLocation _returnvalue) "TraceTypeQuery2" false (Utilities|Array|MakeArray _returnvalue Target) "None"))
  (return _returnvalue_2))

(fn CheckforModifiers
  (bind _asreaper_game_state (Utilities|Casting|CastToReaperGameState (Game|GetGameState)))
  (if (Variables|/Game/ReaperGameState.ReaperGameState_C|GetWind_Modifier1 _asreaper_game_state)
    (Variables|SpellValues|SetSpellDuration (Variables|SpellValues|GetModifier_Duration)))
  (if (Variables|/Game/ReaperGameState.ReaperGameState_C|GetWind_Modifier2 _asreaper_game_state)
    (Variables|SpellValues|SetKnockbackStrength (Variables|SpellValues|GetModifier_Knockback))))