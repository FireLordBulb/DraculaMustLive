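; BP_SpawnMinions is a Reaper spell actor that spawns a group of minions, then destroys itself.
; On BeginPlay it reads MinionModifier1 from ReaperGameState to override the spawn count and aligns itself to the player's rotation.
; Downward traces lower five spawn point components to just above the surface hit.
; Minions then spawn at those points, raised by their half height and facing the player's direction.
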(event EventBeginPlay
  (CallFunction|CheckforModifiers)
  (Variables|Default|SetSpawnPoints (Utilities|Array|MakeArray (Variables|Default|GetSpawnPoint1) (Variables|Default|GetSpawnPoint2) (Variables|Default|GetSpawnPoint3) (Variables|Default|GetSpawnPoint4) (Variables|Default|GetSpawnPoint5)))
  (bind _output_get (Variables|Default|SetPlayerRotation (Transformation|GetActorRotation (Game|Player|GetPlayerPawn 0))))
  (Transformation|SetActorRotation _output_get)
  (Utilities|FlowControl|Sequence
    (:then_0
      (for _array_element (Variables|Default|GetSpawnPoints)
        (bind _outhit (Collision|LineTraceByChannel (Transformation|GetWorldLocation _array_element) (+ (Transformation|GetWorldLocation _array_element) (* (Math|Vector|GetUpVector (Transformation|GetWorldRotation _array_element)) -1e+03)) "TraceTypeQuery1" false 0 "ForDuration"))
        (if (.bBlockingHit (Collision|BreakHitResult _outhit))
          (Transformation|SetRelativeTransform _array_element (Math|Transform|MakeTransform (Math|Vector|MakeVector (.x (.location (Transformation|GetRelativeTransform _array_element))) (.y (.location (Transformation|GetRelativeTransform _array_element))) (+ (- (.z (.location (Transformation|GetRelativeTransform _array_element))) (.Distance (Collision|BreakHitResult _outhit))) 1e+01)) "0, 0, 0" "1.000000,1.000000,1.000000") false false)
          (else
            (Development|PrintText "Hello")))))
    (:then_1
      (CallFunction|SpawnAmountOfMinions))
    (:then_2
      (Actor|DestroyActor))))

(fn ConstructionScript)

(fn SpawnAmountOfMinions
  (for _index (range 0 (- (Variables|Default|GetSpawnAmount) 1))
    (Game|SpawnActorfromClass (Variables|Default|GetMinionClass) (Math|Transform|MakeTransform (+ (Transformation|GetWorldLocation (Utilities|Array|Get(acopy) (Variables|Default|GetSpawnPoints) _index)) (Math|Vector|MakeVector 0.0 0.0 (Variables|Default|GetMinionHalfHeight))) (Variables|Default|GetPlayerRotation) "1.000000,1.000000,1.000000") "AdjustIfPossibleButAlwaysSpawn" "MultiplyWithRoot" 0 0)))

(fn CheckforModifiers
  (bind _asreaper_game_state (Utilities|Casting|CastToReaperGameState (Game|GetGameState)))
  (if (Variables|/Game/ReaperGameState.ReaperGameState_C|GetMinion_Modifier1 _asreaper_game_state)
    (Variables|Default|SetSpawnAmount (Variables|Default|GetModifier_SpawnAmount))))